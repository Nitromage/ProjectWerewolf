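; Base building actor driven by BuildingDatabase, with health, upgrades, selling and placement overlap checks.
; Set applies the row's mesh, scale, costs and health; upgrades check player resources and owned-building requirements, then spend gold and wood.
; Tick flags blocked placement from overlaps, except index 8 (fishing net), which needs water-tagged meshes.
; Selling replaces the building with an item; damage is authority-only, and the health widget shows for the local owner.
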(event `SerSetHealth`
  (params (Max :type Integer) (Current :type Integer))
  (set `self.MaxHealthHealth` Max)
  (set `self.Health` Current))

(event `self.ReceiveBeginPlay`)

(event `owning`
  (params (actor :type "Actor Object Reference"))
  (bind _asthird_person_character (cast `/Game/ThirdPersonBP/Blueprints/ThirdPersonCharacter` actor))
  (`/Engine/EditorBlueprintResources/StandardMacros.IsValid` _asthird_person_character
    (:`Is Valid`
      (if (`Pawn.IsLocallyControlled` _asthird_person_character)
        (bind _returnvalue (`|CreateWidget` "/Game/Levels/Steffen/Widgets/ingameMenues/BuildingHealth.BuildingHealth_C" null self (`self.RealName`)))
        (bind _output_get (set `self.HealthWB` _returnvalue))
        (`UserWidget.AddToViewport` _output_get 0)
        (else
          ;[1 1 1] Box Collision Widget Health Bar
          (`VictoryBPFunctionLibrary.RemoveAllWidgetsOfClass` "/Game/Levels/Steffen/Widgets/ingameMenues/BuildingHealth.BuildingHealth_C"))))))

(event `self.Box.OnComponentBeginOverlap`
  (params (OverlappedComponent :type "PrimitiveComponent Object Reference") (OtherActor :type "Actor Object Reference") (OtherComp :type "PrimitiveComponent Object Reference") (OtherBodyIndex :type Integer) (bFromSweep :type Boolean) (SweepResult :type "HitResult Structure (by ref)"))
  ;[1 1 1] Box Collision Widget Health Bar
)

(event `self.ReceiveTick`
  (params (DeltaSeconds :type "Float (single-precision)"))
  (if (== (`self.BuildingIndex`) 8)
    (set `self.HitWater?` false)
    (for _array_element (`self.GetOverlappingActors` "/Script/Engine.StaticMeshActor")
      (bind _componenttags (`ActorComponent.ComponentTags` (`self.GetComponentByClass` _array_element "/Script/Engine.StaticMeshComponent")))
      (if (`KismetArrayLibrary.Array_IsValidIndex` _componenttags)
        (if (== (`|GetArrayItem` _componenttags) "Water")
          (set `self.HitWater?` true)
          (break)
          (else
            _)))
      (set `self.HitWater?` false))
    (if (`self.HitWater?`)
      (set `self.IsOverlapping` false :!label _label)
      (else
        (set `self.IsOverlapping` true :!label _label_2)))
    (elif (> (`KismetArrayLibrary.Array_Length` (`self.GetOverlappingActors` "/Script/Engine.Actor")) 0)
      (goto _label_2)
      (elif (> (`KismetArrayLibrary.Array_Length` (`self.GetOverlappingActors` "/Script/Engine.StaticMeshActor")) 0)
        (goto _label_2)
        (else
          (goto _label))))))

(event `self.Box.OnComponentEndOverlap`
  (params (OverlappedComponent :type "PrimitiveComponent Object Reference") (OtherActor :type "Actor Object Reference") (OtherComp :type "PrimitiveComponent Object Reference") (OtherBodyIndex :type Integer))
  ;[1 1 1] Box Collision Widget Health Bar
)

(event `AnotherOwning`
  (params (NewParam :type "Actor Object Reference"))
  (bind _asthird_person_character (cast `/Game/ThirdPersonBP/Blueprints/ThirdPersonCharacter` NewParam))
  (`/Engine/EditorBlueprintResources/StandardMacros.IsValid` _asthird_person_character
    (:`Is Valid`
      (if (`Pawn.IsLocallyControlled` _asthird_person_character)
        _
        (else
          _))
      (`VictoryBPFunctionLibrary.RemoveAllWidgetsOfClass` "/Game/Levels/Steffen/Widgets/ingameMenues/BuildingHealth.BuildingHealth_C"))))

(event `self.ReceiveAnyDamage`
  (params (Damage :type "Float (single-precision)") (DamageType :type "DamageType Object Reference") (InstigatedBy :type "Controller Object Reference") (DamageCauser :type "Actor Object Reference"))
  ;[1 0 0] On take Dmg
  (`self.TakeDamage` Damage))

(fn `BuyUpgrade`
  (bind _asthird_person_character (cast `/Game/ThirdPersonBP/Blueprints/ThirdPersonCharacter` (`GameplayStatics.GetPlayerCharacter` 0)))
  (set `/Game/ThirdPersonBP/Blueprints/ThirdPersonCharacter.WoodCount` (- (`/Game/ThirdPersonBP/Blueprints/ThirdPersonCharacter.WoodCount` _asthird_person_character) (`self.WoodUpgradeCost`)) _asthird_person_character)
  (set `/Game/ThirdPersonBP/Blueprints/ThirdPersonCharacter.GoldCount` (- (`/Game/ThirdPersonBP/Blueprints/ThirdPersonCharacter.GoldCount` _asthird_person_character) (`self.GoldUpgradeCost`)) _asthird_person_character))

(fn `CheckOverlapping`
  (returns (`Overlapping?` :type Boolean))
  (if (> (`KismetArrayLibrary.Array_Length` (`self.GetOverlappingActors` "/Script/Engine.Actor")) 0)
    _
    (elif (> (`KismetArrayLibrary.Array_Length` (`self.GetOverlappingActors` "/Script/Engine.StaticMeshActor")) 0)
      _
      (else
        (return false))))
  (return true))

(fn `CheckUpgrade`
  (returns (`CanUpgrade?` :type Boolean))
  (locals (`CanAfford?` :type Boolean) (`Upgrade?` :type Boolean :default true) (`HasCheckedOwnedBuildings?` :type Boolean))
  (bind _asthird_person_character (cast `/Game/ThirdPersonBP/Blueprints/ThirdPersonCharacter` (`GameplayStatics.GetPlayerCharacter` 0)))
  (if (and (>= (`/Game/ThirdPersonBP/Blueprints/ThirdPersonCharacter.WoodCount` _asthird_person_character) (`self.WoodUpgradeCost`)) (>= (`/Game/ThirdPersonBP/Blueprints/ThirdPersonCharacter.GoldCount` _asthird_person_character) (`self.GoldUpgradeCost`)))
    (bind _returnvalue (`|GetDataTableRow` "/Game/Blueprints/Patrick/Buildings/BuildingDatabase.BuildingDatabase" (`KismetStringLibrary.Conv_StringToName` (`KismetStringLibrary.Conv_IntToString` (`self.BuildingIndex`))))
      (:`then`
        (`KismetSystemLibrary.PrintString` (`KismetStringLibrary.Concat_StrStr` "Checking building index - " (`KismetStringLibrary.Conv_IntToString` (`self.BuildingIndex`))))
        (bind (_buildingindex _level) (break `/Game/Blueprints/Patrick/Buildings/BuildingRequirements` (`|GetArrayItem` (`.BuildingRequirements_87_39C5126042AA7A1A428D8FBF60D2B184` (break `/Game/Blueprints/Patrick/Buildings/BuildingStruct` _returnvalue)) (`self.CurrentLevel`))))
        (`KismetSystemLibrary.PrintString` (`KismetStringLibrary.Concat_StrStr` "Building requires " (`KismetStringLibrary.Conv_IntToString` (`KismetArrayLibrary.Array_Length` _buildingindex)) " number of buildings"))
        (for (_array_element _array_index) _buildingindex
          (set `local.HasCheckedOwnedBuildings?` true)
          (`KismetSystemLibrary.PrintString` (`KismetStringLibrary.Concat_StrStr` "Checking owned building - " (`KismetStringLibrary.Conv_IntToString` _array_element)))
          (bind _asthird_person_character_2 (cast `/Game/ThirdPersonBP/Blueprints/ThirdPersonCharacter` (`GameplayStatics.GetPlayerCharacter` 0)))
          (bind (_buildingindex_2 _level_2) (break `/Game/Blueprints/Patrick/Buildings/BuildingRequirements` (`/Game/ThirdPersonBP/Blueprints/ThirdPersonCharacter.OwnedBuildings` _asthird_person_character_2)))
          (if (and (`KismetArrayLibrary.Array_Contains` _buildingindex_2 _array_element) (`KismetArrayLibrary.Array_Contains` _level_2 (`|GetArrayItem` _level _array_index)))
            (set `local.Upgrade?` true)
            (`KismetSystemLibrary.PrintString` "Can upgrade")
            (else
              (set `local.Upgrade?` false)
              (`KismetSystemLibrary.PrintString` "Doesn't own correct buildings"))))
        (if (`local.HasCheckedOwnedBuildings?`)
          (return (`local.Upgrade?`))
          (else
            (`KismetSystemLibrary.PrintString` "Doesn't own any buildings")))))))

(fn `SellBuilding`
  (params (ItemIndex :type Integer))
  (bind _returnvalue (`|GetDataTableRow` "/Game/Blueprints/Patrick/Items/Item_Database.Item_Database" (`KismetStringLibrary.Conv_StringToName` (`KismetStringLibrary.Conv_IntToString` ItemIndex)))
    (:`then`
      (bind _returnvalue_2 (`|SpawnActorFromClass` "/Game/Blueprints/Patrick/Items/Item.Item_C" (`KismetMathLibrary.MakeTransform` (`KismetMathLibrary.MakeVector` (.x (.location (`self.GetTransform`))) (.y (.location (`self.GetTransform`))) 200.0) (.rotation (`self.GetTransform`)) (`.Scale_56_49A000414293555438723B8859A2B073` (break `/Game/Blueprints/Patrick/Items/ItemStruct` _returnvalue))) "Undefined" "OverrideRootScale" null null))
      (bind _returnvalue_3 (`|GetDataTableRow` "/Game/Blueprints/Patrick/Buildings/BuildingDatabase.BuildingDatabase" (`KismetStringLibrary.Conv_StringToName` (`KismetStringLibrary.Conv_IntToString` (`self.BuildingIndex`))))
        (:`then`
          (bind (_name _meshes _scale _upgradecostgold _upgradecostwood _buildingrequirements _buygoldcost _buywoodcost _canupgrade_ _hasshop_ _shopitems _maxlevel _itemindex) (break `/Game/Blueprints/Patrick/Buildings/BuildingStruct` _returnvalue_3))
          (bind _returnvalue_4 (`|GetDataTableRow` "/Game/Blueprints/Patrick/Items/Item_Database.Item_Database" (`KismetStringLibrary.Conv_StringToName` (`KismetStringLibrary.Conv_IntToString` _itemindex)))
            (:`then`
              (`StaticMeshComponent.SetStaticMesh` (`/Game/Blueprints/Patrick/Items/Item.StaticMesh` _returnvalue_2) (`.Mesh_70_1D882473448640A8EF416BBBBB35CE35` (break `/Game/Blueprints/Patrick/Items/ItemStruct` _returnvalue_4)))
              (set `/Game/Blueprints/Patrick/Items/Item.ItemIndex` _itemindex _returnvalue_2)
              (`self.K2_DestroyActor`))))))))

(fn `Set`
  (params (BuildingIndex :type Integer))
  (bind _currentlevel (`self.CurrentLevel`))
  (bind _returnvalue (`|GetDataTableRow` "/Game/Blueprints/Patrick/Buildings/BuildingDatabase.BuildingDatabase" (`KismetStringLibrary.Conv_StringToName` (`KismetStringLibrary.Conv_IntToString` BuildingIndex)))
    (:`then`
      (bind (_name _meshes _scale _upgradecostgold _upgradecostwood _buildingrequirements _buygoldcost _buywoodcost _canupgrade_ _hasshop_ _shopitems _maxlevel _itemindex _health) (break `/Game/Blueprints/Patrick/Buildings/BuildingStruct` _returnvalue))
      (set `self.Name` (`KismetStringLibrary.Conv_StringToName` (`KismetStringLibrary.Concat_StrStr` "Level " (`KismetStringLibrary.Conv_IntToString` (+ (`self.CurrentLevel`) 1)) " " _name)))
      (`StaticMeshComponent.SetStaticMesh` (`self.StaticMesh`) (`|GetArrayItem` _meshes _currentlevel))
      (set `self.GoldUpgradeCost` (`|GetArrayItem` _upgradecostgold _currentlevel))
      (set `self.WoodUpgradeCost` (`|GetArrayItem` _upgradecostwood _currentlevel))
      (set `self.HasShop?` _hasshop_)
      (`SceneComponent.SetWorldScale3D` (`self.StaticMesh`) (`|GetArrayItem` _scale _currentlevel))
      (set `self.BuildingIndex` BuildingIndex)
      (set `self.MaxLevel` _maxlevel)
      (`self.SerSetHealth` _health _health)
      (set `self.Ready?` true)
      (set `self.RealName` (`KismetTextLibrary.Conv_NameToText` (`KismetStringLibrary.Conv_StringToName` _name))))))

(fn `SetInfo`
  (params (WoodBuyCost :type Integer) (GoldBuyCost :type Integer) (`HasShop?` :type Boolean) (WoodUpgradeCost :type Integer) (GoldUpgradeCost :type Integer) (WoodSellValue :type Integer) (GoldSellValue :type Integer) (Name :type Name) (MaxLevel :type Integer) (NewShopItems :type "Array of /Game/Blueprints/Patrick/Items/ItemStackStruct Structure"))
  (set `self.WoodBuyCost` WoodBuyCost)
  (set `self.GoldBuyCost` GoldBuyCost)
  (set `self.HasShop?` `HasShop?`)
  (set `self.WoodUpgradeCost` WoodUpgradeCost)
  (set `self.GoldUpgradeCost` GoldUpgradeCost)
  (set `self.WoodSellValue` WoodSellValue)
  (set `self.GoldSellValue` GoldSellValue)
  (set `self.Name` Name)
  (set `self.MaxLevel` MaxLevel)
  (set `self.NewShopItems` NewShopItems))

(fn `TakeDamage`
  (params (Dmg :type "Float (double-precision)"))
  (`/Engine/EditorBlueprintResources/ActorMacros.Switch Has Authority`
    (:`Authority`
      (bind _output_get (set `self.Health` (- (`self.Health`) (`KismetMathLibrary.FTrunc` Dmg))))
      (`KismetSystemLibrary.PrintString` (`KismetStringLibrary.Conv_IntToString` _output_get)))))

(fn `UpgradeBuilding`
  (bind _asthird_person_character (cast `/Game/ThirdPersonBP/Blueprints/ThirdPersonCharacter` (`GameplayStatics.GetPlayerCharacter` 0)))
  (set `/Game/ThirdPersonBP/Blueprints/ThirdPersonCharacter.GoldCount` (- (`/Game/ThirdPersonBP/Blueprints/ThirdPersonCharacter.GoldCount` _asthird_person_character) (`self.GoldUpgradeCost`)) _asthird_person_character)
  (set `/Game/ThirdPersonBP/Blueprints/ThirdPersonCharacter.WoodCount` (- (`/Game/ThirdPersonBP/Blueprints/ThirdPersonCharacter.WoodCount` _asthird_person_character) (`self.WoodUpgradeCost`)) _asthird_person_character)
  (`/Engine/EditorBlueprintResources/StandardMacros.IncrementInt` (`self.CurrentLevel`)
    (:`  `
      (`self.Set` (`self.BuildingIndex`)))))

(fn `UserConstructionScript`)