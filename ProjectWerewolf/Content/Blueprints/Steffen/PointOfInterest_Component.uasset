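; PointOfInterest_Component is an actor component apparently meant to register its owner as a point of interest on the player's minimap.
; BeginPlay only starts a short Delay with nothing wired after it, so registration never runs.
; The disconnected logic takes the last controller in ThirdPersonGameMode's AllPlayerControllers, casts its pawn to ThirdPersonCharacter, and passes the owner to the HUD minimap's AddPOI.
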(event `self.ReceiveBeginPlay`
  (`KismetSystemLibrary.Delay` 0.2))