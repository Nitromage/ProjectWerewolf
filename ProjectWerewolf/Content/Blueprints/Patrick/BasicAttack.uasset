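; BasicAttack is a short-lived ability actor that detects what it overlaps during an attack.
; On overlap it ignores actors tagged Ability and its own instigator, then checks for the Attackable tag.
; The hit result is only printed as a debug string, with no damage applied.
; Tick accumulates a timer and destroys the actor once AbilityTime is reached.
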(event `self.ReceiveActorBeginOverlap`
  (params (OtherActor :type "Actor Object Reference"))
  (if (`self.ActorHasTag` OtherActor "Ability")
    _
    (elif (!= (`self.GetInstigator`) OtherActor)
      (if (`self.ActorHasTag` OtherActor "Attackable")
        (`KismetSystemLibrary.PrintString` "Damaging Actor")
        (else
          (`KismetSystemLibrary.PrintString` "Actor is not attackable"))))))

(event `self.ReceiveTick`
  (params (DeltaSeconds :type "Float (single-precision)"))
  (set `self.Timer` (+ (`self.Timer`) DeltaSeconds))
  (if (>= (`self.Timer`) (`self.AbilityTime`))
    (`self.K2_DestroyActor`)))

(fn `UserConstructionScript`)