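; Wall is an actor Blueprint that keeps the Structure IsOverlapping flag in sync with its overlaps.
; Begin and end overlap events cast self to Structure and set the flag true or false, so any single end clears it without checking remaining overlaps.
; An unconnected polling branch using GetOverlappingActors on the parent actor never runs, Tick is empty, and the construction script only calls its parent.
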(event `self.ReceiveActorEndOverlap`
  (params (OtherActor :type "Actor Object Reference"))
  (bind _asstructure (cast `/Game/Blueprints/Patrick/Structure` self))
  (set `/Game/Blueprints/Patrick/Structure.IsOverlapping` false _asstructure))

(event `self.ReceiveActorBeginOverlap`
  (params (OtherActor :type "Actor Object Reference"))
  (bind _asstructure (cast `/Game/Blueprints/Patrick/Structure` self))
  (set `/Game/Blueprints/Patrick/Structure.IsOverlapping` true _asstructure))

(event `self.ReceiveTick`
  (params (DeltaSeconds :type "Float (single-precision)")))

(fn `UserConstructionScript`
  (`parent.UserConstructionScript`))