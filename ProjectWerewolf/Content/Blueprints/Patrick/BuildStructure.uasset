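; Building placement component that lets the player preview, rotate and build structures, with server events handling spawning.
; A server-spawned preview returns to the owning client, where Tick moves it to Landscape hits from a control-rotation trace.
; Gold and wood costs from BuildingDatabase plus an overlap check set CanBuild, swapping original materials with NoBuildMat.
; ServerBuild spawns the final Structure or FarmStructure according to the item table's farming flag.
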(event `Ser_build`
  (params (Player :type "Actor Object Reference") (BuildingIndex :type Integer) (Transform :type "Transform Structure"))
  (`self.ServerBuild` Player BuildingIndex Transform))

(event `self.ReceiveTick`
  (params (DeltaSeconds :type "Float (single-precision)"))
  ;[1 1 1] Update Selected Structure
  (`self.UpdateShowbuilding`))

(event `ServerSpawnCall`
  (params (Transform :type "Transform Structure") (BuildingIndex :type Integer))
  ;[1 1 1] Show Buildings
  ;;[1 1 1] Server
  (bind _returnvalue (`|SpawnActorFromClass` "/Game/Blueprints/Patrick/Buildings/Structure.Structure_C" Transform "Undefined" "OverrideRootScale" null null))
  (`self.OwningClient` _returnvalue BuildingIndex)
  (`PrimitiveComponent.SetCollisionProfileName` (`/Game/Blueprints/Patrick/Buildings/Structure.StaticMesh` _returnvalue) "OverlapAllDynamic"))

(event `OwningClient`
  (params (CurrentStructure :type "Actor Object Reference") (BuildingIndex :type Integer))
  ;[1 1 1] Show Buildings
  ;;[1 1 1] Client
  (bind _output_get (set `self.CurrentStructure` CurrentStructure))
  (bind _asstructure (cast `/Game/Blueprints/Patrick/Buildings/Structure` _output_get :!pure true))
  (`/Game/Blueprints/Patrick/Buildings/Structure.Set` _asstructure BuildingIndex)
  (set `/Game/Blueprints/Patrick/Buildings/Structure.IsBuild?` false _asstructure)
  (set `self.StructureMats` (`MeshComponent.GetMaterials` (`Actor.GetComponentByClass` _output_get "/Script/Engine.StaticMeshComponent"))))

(event `ClearDataServer`
  ;[1 1 1] Show Buildings
  (`self.ClearData`))

(event `ServerSet`
  (params (target :type "/Game/Blueprints/Patrick/BuildStructure Object Reference") (Index :type Integer) (CurrentStructure :type "/Game/Blueprints/Patrick/Buildings/Structure Object Reference") (Component :type "Actor Object Reference"))
  ;[1 1 1] Show Buildings
)

(event `UpdateBuildingPosServer`
  (params (Target :type "Actor Object Reference") (Transform :type "Transform Structure"))
  ;[1 1 1] Server
  (`Actor.K2_SetActorTransform` Target Transform false false))

(event `OwningUpdate`
  (bind _asthird_person_character (cast `/Game/ThirdPersonBP/Blueprints/ThirdPersonCharacter` (`GameplayStatics.GetPlayerCharacter` 0) :!pure true))
  ;[1 1 1] Client
  (bind _canbuild_ (`self.CheckCost` (`/Game/ThirdPersonBP/Blueprints/ThirdPersonCharacter.GoldCount` _asthird_person_character) (`/Game/ThirdPersonBP/Blueprints/ThirdPersonCharacter.WoodCount` _asthird_person_character)))
  (if _canbuild_
    (bind _canbuild__2 (`self.CheckOverlapping`))
    (if _canbuild__2
      (set `/Game/ThirdPersonBP/Blueprints/ThirdPersonCharacter.CanBuild` true _asthird_person_character)
      (else
        (set `/Game/ThirdPersonBP/Blueprints/ThirdPersonCharacter.CanBuild` false _asthird_person_character)))
    (else
      (set `/Game/ThirdPersonBP/Blueprints/ThirdPersonCharacter.CanBuild` false _asthird_person_character)))
  (`self.SetMaterial` (`/Game/ThirdPersonBP/Blueprints/ThirdPersonCharacter.CanBuild` _asthird_person_character)))

(fn `CheckCost`
  (params (PlayerGold :type Integer) (PlayerWood :type Integer))
  (returns (`CanBuild?` :type Boolean))
  (bind _asstructure (cast `/Game/Blueprints/Patrick/Buildings/Structure` (`self.CurrentStructure`)))
  (cast `/Game/ThirdPersonBP/Blueprints/ThirdPersonCharacter` (`self.GetOwner`))
  (bind _returnvalue (`|GetDataTableRow` "/Game/Blueprints/Patrick/Buildings/BuildingDatabase.BuildingDatabase" (`KismetStringLibrary.Conv_StringToName` (`KismetStringLibrary.Conv_IntToString` (`/Game/Blueprints/Patrick/Buildings/Structure.BuildingIndex` _asstructure))))
    (:`then`
      (bind (_name _meshes _scale _upgradecostgold _upgradecostwood _buildingrequirements _buygoldcost _buywoodcost) (break `/Game/Blueprints/Patrick/Buildings/BuildingStruct` _returnvalue))
      (if (and (>= PlayerWood _buywoodcost) (>= PlayerGold _buygoldcost))
        (return true)
        (else
          (return false))))))

(fn `CheckOverlapping`
  (returns (`CanBuild?` :type Boolean))
  (bind _asstructure (cast `/Game/Blueprints/Patrick/Buildings/Structure` (`self.CurrentStructure`)))
  (if (`/Game/Blueprints/Patrick/Buildings/Structure.IsOverlapping` _asstructure)
    (return false)
    (else
      (return true))))

(fn `ClearData`
  (bind _asthird_person_character (cast `/Game/ThirdPersonBP/Blueprints/ThirdPersonCharacter` (`GameplayStatics.GetPlayerCharacter` 0)))
  (set `/Game/ThirdPersonBP/Blueprints/ThirdPersonCharacter.IsBuilding` false _asthird_person_character)
  (set `/Game/ThirdPersonBP/Blueprints/ThirdPersonCharacter.CanBuild` false _asthird_person_character)
  (`Actor.K2_DestroyActor` (`self.CurrentStructure`)))

(fn `IsValid`
  (params (NewParam :type "Actor Object Reference"))
  (if (`KismetSystemLibrary.IsValid` NewParam)
    (return)
    (else
      (`KismetSystemLibrary.PrintString` "not valid"))))

(fn `Rotate`
  (params (IsRotatingRight :type Boolean))
  (locals (RotateFactor :type "Float (double-precision)" :default 10.0))
  (bind _currentstructure (`self.CurrentStructure`))
  (bind _currentstructure_2 (`self.CurrentStructure`))
  (if IsRotatingRight
    (`Actor.K2_SetActorRotation` _currentstructure_2 (`KismetMathLibrary.MakeRotator` (.roll (`Actor.K2_GetActorRotation` _currentstructure_2)) (.pitch (`Actor.K2_GetActorRotation` _currentstructure_2)) (+ (.yaw (`Actor.K2_GetActorRotation` _currentstructure_2)) (`local.RotateFactor`))) false)
    (else
      (`Actor.K2_SetActorRotation` _currentstructure (`KismetMathLibrary.MakeRotator` (.roll (`Actor.K2_GetActorRotation` _currentstructure)) (.pitch (`Actor.K2_GetActorRotation` _currentstructure)) (- (.yaw (`Actor.K2_GetActorRotation` _currentstructure)) (`local.RotateFactor`))) false))))

(fn `ServerBuild`
  (params (Player :type "Actor Object Reference") (BuildingIndex :type Integer) (Transform :type "Transform Structure"))
  (locals (Class :type "Actor Class Reference"))
  (bind _returnvalue (`|GetDataTableRow` "/Game/Blueprints/Patrick/Buildings/BuildingDatabase.BuildingDatabase" (`KismetStringLibrary.Conv_StringToName` (`KismetStringLibrary.Conv_IntToString` BuildingIndex)))
    (:`then`
      (bind _returnvalue_2 (`|GetDataTableRow` "/Game/Blueprints/Patrick/Items/Item_Database.Item_Database" (`KismetStringLibrary.Conv_StringToName` (`KismetStringLibrary.Conv_IntToString` (`.ItemIndex_82_F114134544E054E752B4CCAA4C00EEB6` (break `/Game/Blueprints/Patrick/Buildings/BuildingStruct` _returnvalue)))))
        (:`then`
          (if (`.IsFarmingItem_58_964725D54E52A0FF7B858D8DEC75C6EB` (break `/Game/Blueprints/Patrick/Items/ItemStruct` _returnvalue_2))
            (set `local.Class` "/Game/Blueprints/Patrick/Buildings/FarmStructure.FarmStructure_C")
            (else
              (set `local.Class` "/Game/Blueprints/Patrick/Buildings/Structure.Structure_C")))
          (bind _returnvalue_3 (`|SpawnActorFromClass` (`local.Class`) Transform "Undefined" "OverrideRootScale" Player null))
          (bind _asstructure (cast `/Game/Blueprints/Patrick/Buildings/Structure` _returnvalue_3)
            (:`then`
              (set `/Game/Blueprints/Patrick/Buildings/Structure.IsBuild?` true _asstructure)
              (`KismetSystemLibrary.PrintString` "Spawning structure" true true (struct :`G` 0.66 :`B` 1.0 :`A` 1.0) 5.0)
              (`/Game/Blueprints/Patrick/Buildings/Structure.Set` _asstructure BuildingIndex)
              (`self.SetIsReplicated` (`/Game/Blueprints/Patrick/Buildings/Structure.StaticMesh` _asstructure) true))
            (:`CastFailed`
              (bind _asfarm_structure (cast `/Game/Blueprints/Patrick/Buildings/FarmStructure` _returnvalue_3)
                (:`then`
                  (`KismetSystemLibrary.PrintString` "Spawning farm" true true (struct :`G` 0.66 :`B` 1.0 :`A` 1.0) 5.0)
                  (`/Game/Blueprints/Patrick/Buildings/FarmStructure.Set` _asfarm_structure BuildingIndex)
                  (`self.SetIsReplicated` (`/Game/Blueprints/Patrick/Buildings/FarmStructure.StaticMesh` _asfarm_structure) true))
                (:`CastFailed`
                  (`KismetSystemLibrary.PrintString` "Unknown building" true true (struct :`G` 0.66 :`B` 1.0 :`A` 1.0) 5.0))))))))))

(fn `SetMaterial`
  (params (`CanBuild?` :type Boolean))
  (bind _returnvalue (`Actor.GetComponentByClass` (`self.CurrentStructure`) "/Script/Engine.StaticMeshComponent"))
  (bind _returnvalue_2 (`MeshComponent.GetMaterials` (`Actor.GetComponentByClass` (`self.CurrentStructure`) "/Script/Engine.StaticMeshComponent")))
  (if `CanBuild?`
    (for _index (range (`KismetArrayLibrary.Array_Length` _returnvalue_2))
      (bind _output (`|GetArrayItem` (`self.StructureMats`) _index))
      (if (!= (`|GetArrayItem` _returnvalue_2 _index) _output)
        (`PrimitiveComponent.SetMaterial` (`Actor.GetComponentByClass` (`self.CurrentStructure`) "/Script/Engine.StaticMeshComponent") _index _output)))
    (else
      (for _array_element (`MeshComponent.GetMaterials` (`Actor.GetComponentByClass` (`self.CurrentStructure`) "/Script/Engine.StaticMeshComponent"))
        (if (!= _array_element (`self.NoBuildMat`))
          (for _index_2 (range (+ (`KismetArrayLibrary.Array_Length` (`MeshComponent.GetMaterials` _returnvalue)) 1))
            (`PrimitiveComponent.SetMaterial` _returnvalue _index_2 (`self.NoBuildMat`))))))))

(fn `ShowBuild`
  (params (BuildingIndex :type Integer))
  (bind _asthird_person_character (cast `/Game/ThirdPersonBP/Blueprints/ThirdPersonCharacter` (`GameplayStatics.GetPlayerCharacter` 0) :!pure true))
  ;[1 1 1] Start Showing Structure Run from widgets
  (set `/Game/ThirdPersonBP/Blueprints/ThirdPersonCharacter.IsBuilding` true _asthird_person_character)
  (`self.ServerSpawnCall` (`KismetMathLibrary.MakeTransform` (`KismetMathLibrary.MakeVector` (.x (+ (.location (`Actor.GetTransform` _asthird_person_character)) (* (`KismetMathLibrary.GetForwardVector` (`Pawn.GetControlRotation` _asthird_person_character)) (`/Game/ThirdPersonBP/Blueprints/ThirdPersonCharacter.BuildDistance` _asthird_person_character)))) (.y (+ (.location (`Actor.GetTransform` _asthird_person_character)) (* (`KismetMathLibrary.GetForwardVector` (`Pawn.GetControlRotation` _asthird_person_character)) (`/Game/ThirdPersonBP/Blueprints/ThirdPersonCharacter.BuildDistance` _asthird_person_character)))) 100.0) (.rotation (`Actor.GetTransform` _asthird_person_character)) (.scale (`Actor.GetTransform` _asthird_person_character))) BuildingIndex))

(fn `UpdateShowbuilding`
  (bind _returnvalue (`GameplayStatics.GetPlayerCharacter` 0))
  (bind _currentstructure (`self.CurrentStructure`))
  (bind _returnvalue_2 (`Actor.K2_GetActorLocation` _returnvalue))
  (bind _asthird_person_character (cast `/Game/ThirdPersonBP/Blueprints/ThirdPersonCharacter` _returnvalue))
  (if (`/Game/ThirdPersonBP/Blueprints/ThirdPersonCharacter.IsBuilding` _asthird_person_character)
    (if (`KismetSystemLibrary.IsValid` _currentstructure)
      (bind _outhit (`KismetSystemLibrary.LineTraceSingle` _returnvalue_2 (+ _returnvalue_2 (* (`KismetMathLibrary.GetForwardVector` (`Pawn.GetControlRotation` _returnvalue)) 5000.0)) "TraceTypeQuery1" false (`|MakeArray` _currentstructure)))
      (bind (_bblockinghit _binitialoverlap _time _distance _location _impactpoint _normal _impactnormal _physmat _hitactor) (`GameplayStatics.BreakHitResult` _outhit))
      (if _bblockinghit
        (if (<= 0.0 (`/Game/ThirdPersonBP/Blueprints/ThirdPersonCharacter.BuildDistance` _asthird_person_character))
          (cast `Landscape` _hitactor
            (:`then`
              (set `self.CanBuild` true)
              (`Actor.K2_SetActorTransform` (`self.CurrentStructure`) (`KismetMathLibrary.MakeTransform` (`KismetMathLibrary.MakeVector` (.x _location) (.y _location) (.z _location)) (`Actor.K2_GetActorRotation` (`self.CurrentStructure`))) false false)
              (`self.OwningUpdate`))
            (:`CastFailed`
              (set `self.CanBuild` false :!label _label)))
          (else
            (goto _label)))))))