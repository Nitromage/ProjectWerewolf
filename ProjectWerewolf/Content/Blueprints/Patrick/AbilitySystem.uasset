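; AbilitySystem is an owner-attached component that provides the third-person character's basic punch attack.
; BasicAttack spawns an attack actor ahead of the owner along control rotation, at a fixed world height with its Z axis aligned to the aim.
; It sets the character as instigator, plays the punch montage, and returns a hardcoded animation time with the spawned ability box.
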(fn `BasicAttack`
  (returns (AnimationTime :type "Float (double-precision)") (AbilityBox :type "Actor Object Reference"))
  (bind _returnvalue (`self.GetOwner`))
  (bind _returnvalue_2 (`KismetMathLibrary.GetForwardVector` (`Pawn.GetControlRotation` (`Actor.Instigator` _returnvalue))))
  (bind _asthird_person_character (cast `/Game/ThirdPersonBP/Blueprints/ThirdPersonCharacter` (`self.GetOwner`)))
  (bind _returnvalue_3 (`|SpawnActorFromClass` "/Game/Blueprints/Patrick/BasicAttack.BasicAttack_C" (`KismetMathLibrary.MakeTransform` (`KismetMathLibrary.MakeVector` (.x (+ (`Actor.K2_GetActorLocation` _returnvalue) (* _returnvalue_2 300.0))) (.y (+ (`Actor.K2_GetActorLocation` _returnvalue) (* _returnvalue_2 300.0))) 100.0) (`KismetMathLibrary.MakeRotFromZ` _returnvalue_2) (.scale (`Actor.GetTransform` (`self.GetOwner`)))) "Undefined" "OverrideRootScale" null _asthird_person_character))
  (bind _asthird_person_character_2 (cast `/Game/ThirdPersonBP/Blueprints/ThirdPersonCharacter` (`self.GetOwner`)))
  (`Character.PlayAnimMontage` _asthird_person_character_2 "/Game/Blueprints/Patrick/Animations/ArcherAnimations/PunchMontage.PunchMontage" 1.0 "None")
  (return 1.375 _returnvalue_3))