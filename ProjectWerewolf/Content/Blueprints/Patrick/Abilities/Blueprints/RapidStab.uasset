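; Rapid Stab ability actor that shows an aim effect in front of the player character until cast or canceled.
; Left click starts the cooldown and sends cast, damage and stun calls through AbilitySystem for overlapping actors; right click cancels.
; Both clicks remove the aim emitter and disable player input.
; After casting, Tick repeats damage using a modulo timer window, then destroys the actor and restores input when CastTime expires.
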(event `self.ReceiveBeginPlay`
  ;[1 1 1] Spawn Effect
  (bind _returnvalue (`GameplayStatics.SpawnEmitterAtLocation` "/Game/Blueprints/Patrick/Abilities/ParticleSystems/RapidStab_Aim.RapidStab_Aim" (.location (`self.GetTransform`)) (.rotation (`self.GetTransform`)) (.scale (`self.GetTransform`)) false))
  (set `self.VisualEmitter` _returnvalue))

(event `Key|LeftMouseButton`
  (params (Key :type "Key Structure"))
  (bind _overlappingactors (`PrimitiveComponent.GetOverlappingActors` (`self.StaticMesh`) "/Script/Engine.Actor"))
  (bind _asthird_person_character (cast `/Game/ThirdPersonBP/Blueprints/ThirdPersonCharacter` (`GameplayStatics.GetPlayerCharacter` 0) :!pure true))
  (bind _abilitysystem (`/Game/ThirdPersonBP/Blueprints/ThirdPersonCharacter.AbilitySystem` _asthird_person_character))
  ;[1 1 1] Cancel / Cast
  (:`Pressed`
    (`/Game/Blueprints/Patrick/Abilities/Blueprints/AbilitySystem.SetCooldown` _abilitysystem (`self.Cooldown`))
    (set `self.IsCasted?` true)
    (`/Game/Blueprints/Patrick/Abilities/Blueprints/AbilitySystem.Server_Cast` _abilitysystem (`KismetMathLibrary.MakeTransform` (.location (`self.GetTransform`)) (`KismetMathLibrary.MakeRotator` (.roll (.rotation (`self.GetTransform`))) (.pitch (.rotation (`self.GetTransform`))) (+ (.yaw (.rotation (`self.GetTransform`))) 0.0)) (.scale (`self.GetTransform`))) (`|MakeArray` "/Game/Blueprints/Patrick/Abilities/ParticleSystems/RapidStab_Cast.RapidStab_Cast" :!type "ParticleSystem Object Reference"))
    (`/Game/Blueprints/Patrick/Abilities/Blueprints/AbilitySystem.Server_damage` _abilitysystem _asthird_person_character _overlappingactors (`self.Damage`))
    (`/Game/Blueprints/Patrick/Abilities/Blueprints/AbilitySystem.Server_Stun` _abilitysystem _asthird_person_character _overlappingactors 0.0)
    (`self.CleanUp` :!label _label)
    (`self.DisableInput` _asthird_person_character null)))

(event `Key|RightMouseButton`
  (params (Key :type "Key Structure"))
  ;[1 1 1] Cancel / Cast
  (:`Pressed`
    (`/Game/Blueprints/Patrick/Abilities/Blueprints/AbilitySystem.CancelAbility` (`/Game/ThirdPersonBP/Blueprints/ThirdPersonCharacter.AbilitySystem` (cast `/Game/ThirdPersonBP/Blueprints/ThirdPersonCharacter` (`GameplayStatics.GetPlayerCharacter` 0) :!pure true)))
    (goto _label)))

(event `self.ReceiveTick`
  (params (DeltaSeconds :type "Float (single-precision)"))
  (bind _asthird_person_character (cast `/Game/ThirdPersonBP/Blueprints/ThirdPersonCharacter` (`GameplayStatics.GetPlayerCharacter` 0) :!pure true))
  ;[1 1 1] Update
  (if (`self.IsCasted?`)
    (bind _output_get (set `self.Timer` (+ (`self.Timer`) DeltaSeconds)))
    (if (<= _output_get (`self.CastTime`))
      (bind _returnvalue (mod _output_get (`self.DamageInterval`)))
      (if (and (> _returnvalue -0.01) (< _returnvalue 0.01))
        (`/Game/Blueprints/Patrick/Abilities/Blueprints/AbilitySystem.Server_damage` (`/Game/ThirdPersonBP/Blueprints/ThirdPersonCharacter.AbilitySystem` (cast `/Game/ThirdPersonBP/Blueprints/ThirdPersonCharacter` (`GameplayStatics.GetPlayerCharacter` 0) :!pure true)) _asthird_person_character (`PrimitiveComponent.GetOverlappingActors` (`self.StaticMesh`) "/Script/Engine.Actor") (`self.Damage`)))
      (else
        (`self.K2_DestroyActor`)
        (`self.EnableInput` _asthird_person_character null)))
    (else
      (`self.UpdatePosition`))))

(fn `CleanUp`
  (`ActorComponent.K2_DestroyComponent` (`self.VisualEmitter`)))

(fn `MaxLocation`
  (params (PointOne :type "Vector Structure") (PointTwo :type "Vector Structure"))
  (returns (NewPosition :type "Vector Structure"))
  (return (`KismetMathLibrary.MakeVector` (.x (* (`KismetMathLibrary.Normal` (- PointOne PointTwo)) (`self.AbilityRange`))) (.y (* (`KismetMathLibrary.Normal` (- PointOne PointTwo)) (`self.AbilityRange`))) (+ (.z (* (`KismetMathLibrary.Normal` (- PointOne PointTwo)) (`self.AbilityRange`))) 1.0))))

(fn `UpdatePosition`
  (bind _asthird_person_character (cast `/Game/ThirdPersonBP/Blueprints/ThirdPersonCharacter` (`GameplayStatics.GetPlayerCharacter` 0) :!pure true))
  (bind _returnvalue (`KismetMathLibrary.MakeTransform` (`KismetMathLibrary.MakeVector` (.x (+ (* (`KismetMathLibrary.Normal` (`self.GetActorForwardVector` _asthird_person_character)) 200) (.location (`self.GetTransform` _asthird_person_character)))) (.y (+ (* (`KismetMathLibrary.Normal` (`self.GetActorForwardVector` _asthird_person_character)) 200) (.location (`self.GetTransform` _asthird_person_character)))) (- (.z (+ (* (`KismetMathLibrary.Normal` (`self.GetActorForwardVector` _asthird_person_character)) 200) (.location (`self.GetTransform` _asthird_person_character)))) 98.0)) (`KismetMathLibrary.MakeRotator` (.roll (.rotation (`self.GetTransform` _asthird_person_character))) (.pitch (.rotation (`self.GetTransform` _asthird_person_character))) (+ (.yaw (.rotation (`self.GetTransform` _asthird_person_character))) 90.0)) (.scale (`self.GetTransform` _asthird_person_character))))
  (`self.K2_SetActorTransform` _returnvalue)
  (`SceneComponent.K2_SetWorldTransform` (`self.VisualEmitter`) _returnvalue false false))

(fn `UserConstructionScript`)