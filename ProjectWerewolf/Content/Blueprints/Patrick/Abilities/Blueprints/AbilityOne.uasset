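; Ground-targeted area spell actor that shows a circle marker and, once cast, explodes after a timed casting animation.
; Until IsCasted is set, Tick traces from the instigator along control rotation, snapping actor and circle to Landscape hits aligned to the surface normal.
; Clicking spawns a fill effect, while IsCasted starts the montage and timer.
; Completion clears IsCasting and checks overlapping actors' tags, but applies no damage, then destroys itself.
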(event `ScaleOnServer`
  ;[1 1 1] Update Size on the server
  (`self.SetActorScale3D` (* (`self.GetActorScale3D`) (`self.Scale`))))

(event `self.ReceiveBeginPlay`
  ;[1 1 1] Spawn Effect
  (`self.ScaleOnServer`)
  (add `self.OnClicked` (delegate `StartCast`))
  (bind _returnvalue (`GameplayStatics.SpawnEmitterAtLocation` "/Game/Blueprints/Patrick/Abilities/ParticleSystems/CircleParticle.CircleParticle" (.location (`self.GetTransform`)) (.rotation (`self.GetTransform`)) (.scale (`self.GetTransform`))))
  (set `self.ParticleCircle` _returnvalue))

(event `StartCast` :!signature `self.OnClicked`
  (params (TouchedActor :type "Actor Object Reference") (ButtonPressed :type "Key Structure"))
  ;[1 1 1] Start Casting
  (bind _returnvalue (`GameplayStatics.SpawnEmitterAtLocation` "/Game/Blueprints/Patrick/Abilities/ParticleSystems/CircleFillParticle.CircleFillParticle" (`KismetMathLibrary.MakeVector` (.x (.location (`self.GetTransform`))) (.y (.location (`self.GetTransform`))) (- (.z (.location (`self.GetTransform`))) 0.5)) (.rotation (`self.GetTransform`)) (.scale (`self.GetTransform`))))
  (set `self.ParticleFill` _returnvalue))

(event `self.ReceiveTick`
  (params (DeltaSeconds :type "Float (single-precision)"))
  (if (`KismetSystemLibrary.IsValid` (`self.ParticleCircle`))
    (if (`self.IsCasted?`)
      (if (not (`self.HasStartedAnimation?`))
        ;[1 1 1] Cast Animation
        (set `self.HasStartedAnimation?` true)
        (bind _asthird_person_character (cast `/Game/ThirdPersonBP/Blueprints/ThirdPersonCharacter` (`self.GetInstigator`)))
        (`Character.PlayAnimMontage` _asthird_person_character "/Game/Blueprints/Patrick/Animations/SpellCasting/2H_Casting_01.2H_Casting_01" 0.75 "None"))
      ;[1 1 1] Cast Timer
      (bind _output_get (set `self.CastTimer` (+ (`self.CastTimer`) DeltaSeconds)))
      (if (> _output_get (`self.CastTime`))
        ;[1 1 1] Cast Complete
        (`GameplayStatics.SpawnEmitterAtLocation` "/Game/StarterContent/Particles/P_Explosion.P_Explosion" (.location (`self.GetTransform`)) (.rotation (`self.GetTransform`)) (* (.scale (`self.GetTransform`)) 2.0))
        (bind _asthird_person_character_2 (cast `/Game/ThirdPersonBP/Blueprints/ThirdPersonCharacter` (`self.GetInstigator`)))
        (set `/Game/Blueprints/Patrick/Abilities/Blueprints/AbilitySystem.IsCasting?` false (`/Game/ThirdPersonBP/Blueprints/ThirdPersonCharacter.AbilitySystem` _asthird_person_character_2))
        ;[1 1 1] Collision hit
        (for _array_element (`self.GetOverlappingActors` "/Script/Engine.Actor")
          (if (`self.ActorHasTag` _array_element "Ability")
            _
            (elif (!= (`self.GetInstigator`) _array_element)
              (if (not (`self.ActorHasTag` _array_element "Attackable"))
                (`KismetSystemLibrary.PrintString` "Actor is not attackable")))))
        (`self.K2_DestroyActor`)
        (`ActorComponent.K2_DestroyComponent` (`self.ParticleCircle`)))
      (else
        ;[1 1 1] Update Spell Location
        (`self.UpdateSpell`)))))

(fn `UpdateSpell`
  (bind _asthird_person_character (cast `/Game/ThirdPersonBP/Blueprints/ThirdPersonCharacter` (`self.GetInstigator`)))
  (bind _returnvalue (`self.K2_GetActorLocation` _asthird_person_character))
  (bind _outhit (`KismetSystemLibrary.LineTraceSingle` _returnvalue (+ _returnvalue (* (`KismetMathLibrary.GetForwardVector` (`Pawn.GetControlRotation` _asthird_person_character)) (`self.Range`))) "TraceTypeQuery1"))
  (bind (_bblockinghit _binitialoverlap _time _distance _location _impactpoint _normal _impactnormal _physmat _hitactor) (`GameplayStatics.BreakHitResult` _outhit))
  (if _bblockinghit
    (cast `Landscape` _hitactor)
    (bind _returnvalue_2 (`KismetMathLibrary.MakeTransform` (`KismetMathLibrary.MakeVector` (.x _location) (.y _location) (+ (.z _location) 1.0)) (`KismetMathLibrary.MakeRotFromZ` _normal) (`self.GetActorScale3D`)))
    (`self.K2_SetActorTransform` _returnvalue_2)
    (`SceneComponent.K2_SetWorldTransform` (`self.ParticleCircle`) _returnvalue_2 false false)))

(fn `UserConstructionScript`)