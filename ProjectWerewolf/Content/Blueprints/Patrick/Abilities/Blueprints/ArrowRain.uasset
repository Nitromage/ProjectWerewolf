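; Arrow Rain ability actor that previews a ground target circle, then deals area damage once cast.
; Until cast, a control-rotation line trace moves actor and circle emitter, snapping to Landscape normals in range or using MaxLocation beyond it.
; Left click casts through the player's AbilitySystem, right click cancels, and both remove the circle.
; After casting, it sends ServerDamage for overlapping actors every tick until CastTime expires, then destroys itself.
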(event `self.ReceiveBeginPlay`
  ;[1 1 1] Spawn Effect
  (bind _returnvalue (`GameplayStatics.SpawnEmitterAtLocation` "/Game/Blueprints/Patrick/Abilities/ParticleSystems/CircleParticle.CircleParticle" (.location (`self.GetTransform`)) (.rotation (`self.GetTransform`)) (.scale (`self.GetTransform`)) false))
  (set `self.VisualEmitter` _returnvalue))

(event `Key|LeftMouseButton`
  (params (Key :type "Key Structure"))
  ;[1 1 1] Cancel / Cast
  (:`Pressed`
    (set `self.IsCasted?` true)
    (`/Game/Blueprints/Patrick/Abilities/Blueprints/AbilitySystem.Server_Cast` (`/Game/ThirdPersonBP/Blueprints/ThirdPersonCharacter.AbilitySystem` (cast `/Game/ThirdPersonBP/Blueprints/ThirdPersonCharacter` (`GameplayStatics.GetPlayerCharacter` 0) :!pure true)) (`self.GetTransform`) (`|MakeArray` "/Game/Blueprints/Patrick/Abilities/ParticleSystems/ArrowRain_Circle.ArrowRain_Circle" "/Game/Blueprints/Patrick/Abilities/ParticleSystems/ArrowRain_Arrow.ArrowRain_Arrow" :!type "ParticleSystem Object Reference"))
    (`self.CleanUp` :!label _label)))

(event `Key|RightMouseButton`
  (params (Key :type "Key Structure"))
  ;[1 1 1] Cancel / Cast
  (:`Pressed`
    (`/Game/Blueprints/Patrick/Abilities/Blueprints/AbilitySystem.CancelAbility` (`/Game/ThirdPersonBP/Blueprints/ThirdPersonCharacter.AbilitySystem` (cast `/Game/ThirdPersonBP/Blueprints/ThirdPersonCharacter` (`GameplayStatics.GetPlayerCharacter` 0) :!pure true)))
    (goto _label)))

(event `self.ReceiveTick`
  (params (DeltaSeconds :type "Float (single-precision)"))
  ;[1 1 1] Update
  (if (`self.IsCasted?`)
    (bind _output_get (set `self.Timer` (+ (`self.Timer`) DeltaSeconds)))
    (if (<= _output_get (`self.CastTime`))
      (if true
        (`/Game/Blueprints/Patrick/Abilities/Blueprints/AbilitySystem.Server_damage` (`/Game/ThirdPersonBP/Blueprints/ThirdPersonCharacter.AbilitySystem` (cast `/Game/ThirdPersonBP/Blueprints/ThirdPersonCharacter` (`GameplayStatics.GetPlayerCharacter` 0) :!pure true)) (`PrimitiveComponent.GetOverlappingActors` (`self.StaticMesh`) "/Script/Engine.Actor") (`self.Damage`) null))
      (else
        (`self.K2_DestroyActor`)))
    (else
      (`self.UpdatePosition`))))

(fn `CleanUp`
  (`ActorComponent.K2_DestroyComponent` (`self.VisualEmitter`)))

(fn `MaxLocation`
  (params (PointOne :type "Vector Structure") (PointTwo :type "Vector Structure"))
  (returns (NewPosition :type "Vector Structure"))
  (return (`KismetMathLibrary.MakeVector` (.x (* (`KismetMathLibrary.Normal` (- PointOne PointTwo)) (`self.AbilityRange`))) (.y (* (`KismetMathLibrary.Normal` (- PointOne PointTwo)) (`self.AbilityRange`))) (+ (.z (* (`KismetMathLibrary.Normal` (- PointOne PointTwo)) (`self.AbilityRange`))) 1.0))))

(fn `UpdatePosition`
  (bind _returnvalue (`self.GetActorScale3D`))
  (bind _asthird_person_character (cast `/Game/ThirdPersonBP/Blueprints/ThirdPersonCharacter` (`GameplayStatics.GetPlayerCharacter` 0)))
  (bind _returnvalue_2 (`self.K2_GetActorLocation` _asthird_person_character))
  (bind _outhit (`KismetSystemLibrary.LineTraceSingle` _returnvalue_2 (+ _returnvalue_2 (* (`KismetMathLibrary.GetForwardVector` (`Pawn.GetControlRotation` _asthird_person_character)) 5000.0)) "TraceTypeQuery1"))
  (bind (_bblockinghit _binitialoverlap _time _distance _location _impactpoint _normal _impactnormal _physmat _hitactor) (`GameplayStatics.BreakHitResult` _outhit))
  (if _bblockinghit
    (if (> _distance (`self.AbilityRange`))
      ;[1 1 1] Max cast range
      (bind _newposition (`self.MaxLocation` (.location (`self.GetTransform` (cast `/Game/ThirdPersonBP/Blueprints/ThirdPersonCharacter` (`GameplayStatics.GetPlayerCharacter` 0) :!pure true))) _location))
      (bind _returnvalue_3 (`KismetMathLibrary.MakeRotFromZ` _normal))
      (bind _returnvalue_4 (`KismetMathLibrary.MakeTransform` _newposition _returnvalue_3 _returnvalue))
      (`self.K2_SetActorTransform` _returnvalue_4)
      (`SceneComponent.K2_SetWorldTransform` (`self.VisualEmitter`) _returnvalue_4 false false)
      (else
        (cast `Landscape` _hitactor)
        (bind _returnvalue_5 (`KismetMathLibrary.MakeTransform` (`KismetMathLibrary.MakeVector` (.x _location) (.y _location) (+ (.z _location) 1.0)) _returnvalue_3 _returnvalue))
        (`self.K2_SetActorTransform` _returnvalue_5)
        (`SceneComponent.K2_SetWorldTransform` (`self.VisualEmitter`) _returnvalue_5 false false)))))

(fn `UserConstructionScript`)