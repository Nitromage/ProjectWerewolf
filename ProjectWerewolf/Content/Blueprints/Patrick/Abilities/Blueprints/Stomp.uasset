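; Stomp ability actor that previews an area-of-effect circle at the local player's feet until it is cast or cancelled.
; Each tick the actor and its aim-circle emitter follow the player character's transform, lowered to ground level.
; Left click sets the cooldown and asks the player's AbilitySystem to play the Stomp effect, damage and stun mesh-overlapping actors server-side.
; Right click cancels; both paths remove the emitter and destroy the actor.
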(event `self.ReceiveBeginPlay`
  ;[1 1 1] Spawn Effect
  (bind _returnvalue (`GameplayStatics.SpawnEmitterAtLocation` "/Game/Blueprints/Patrick/Abilities/ParticleSystems/AimCircle.AimCircle" (`KismetMathLibrary.MakeVector` (.x (.location (`self.GetTransform`))) (.y (.location (`self.GetTransform`))) 101.0) (.rotation (`self.GetTransform`)) (.scale (`self.GetTransform`)) false))
  (set `self.VisualEmitter` _returnvalue)
  (add `self.OnDestroyed` (delegate `OnDestroyed_Event_0`)))

(event `OnDestroyed_Event_0` :!signature `self.OnDestroyed`
  (params (DestroyedActor :type "Actor Object Reference"))
  (bind _visualemitter (`self.VisualEmitter`))
  ;[1 1 1] Spawn Effect
  (if (`KismetSystemLibrary.IsValid` _visualemitter)
    (`ActorComponent.K2_DestroyComponent` _visualemitter)))

(event `Key|LeftMouseButton`
  (params (Key :type "Key Structure"))
  (bind _overlappingactors (`PrimitiveComponent.GetOverlappingActors` (`self.StaticMesh`) "/Script/Engine.Actor"))
  (bind _asthird_person_character (cast `/Game/ThirdPersonBP/Blueprints/ThirdPersonCharacter` (`GameplayStatics.GetPlayerCharacter` 0) :!pure true))
  (bind _abilitysystem (`/Game/ThirdPersonBP/Blueprints/ThirdPersonCharacter.AbilitySystem` _asthird_person_character))
  ;[1 1 1] Cancel / Cast
  (:`Pressed`
    (`/Game/Blueprints/Patrick/Abilities/Blueprints/AbilitySystem.SetCooldown` _abilitysystem (`self.Cooldown`))
    (set `self.IsCasted?` true)
    (`/Game/Blueprints/Patrick/Abilities/Blueprints/AbilitySystem.Server_Cast` _abilitysystem (`KismetMathLibrary.MakeTransform` (`KismetMathLibrary.MakeVector` (.x (.location (`self.GetTransform`))) (.y (.location (`self.GetTransform`))) 101.0) (.rotation (`self.GetTransform`)) (.scale (`self.GetTransform`))) (`|MakeArray` "/Game/Blueprints/Patrick/Abilities/ParticleSystems/Stomp.Stomp" :!type "ParticleSystem Object Reference"))
    (`/Game/Blueprints/Patrick/Abilities/Blueprints/AbilitySystem.Server_damage` _abilitysystem _asthird_person_character _overlappingactors (`self.Damage`))
    (`/Game/Blueprints/Patrick/Abilities/Blueprints/AbilitySystem.Server_Stun` _abilitysystem _asthird_person_character _overlappingactors (`self.StunTime`))
    (`self.CleanUp` :!label _label)
    (`self.K2_DestroyActor`)))

(event `Key|RightMouseButton`
  (params (Key :type "Key Structure"))
  ;[1 1 1] Cancel / Cast
  (:`Pressed`
    (`/Game/Blueprints/Patrick/Abilities/Blueprints/AbilitySystem.CancelAbility` (`/Game/ThirdPersonBP/Blueprints/ThirdPersonCharacter.AbilitySystem` (cast `/Game/ThirdPersonBP/Blueprints/ThirdPersonCharacter` (`GameplayStatics.GetPlayerCharacter` 0) :!pure true)))
    (goto _label)))

(event `self.ReceiveTick`
  (params (DeltaSeconds :type "Float (single-precision)"))
  ;[1 1 1] Update
  (if (not (`self.IsCasted?`))
    (`self.UpdatePosition`)))

(fn `CleanUp`
  (`ActorComponent.K2_DestroyComponent` (`self.VisualEmitter`)))

(fn `MaxLocation`
  (params (PointOne :type "Vector Structure") (PointTwo :type "Vector Structure"))
  (returns (NewPosition :type "Vector Structure"))
  (return (`KismetMathLibrary.MakeVector` (.x (* (`KismetMathLibrary.Normal` (- PointOne PointTwo)) 0.0)) (.y (* (`KismetMathLibrary.Normal` (- PointOne PointTwo)) 0.0)) (+ (.z (* (`KismetMathLibrary.Normal` (- PointOne PointTwo)) 0.0)) 1.0))))

(fn `UpdatePosition`
  (bind _returnvalue (`KismetMathLibrary.MakeTransform` (`KismetMathLibrary.MakeVector` (.x (.location (`self.GetTransform` (cast `/Game/ThirdPersonBP/Blueprints/ThirdPersonCharacter` (`GameplayStatics.GetPlayerCharacter` 0) :!pure true)))) (.y (.location (`self.GetTransform` (cast `/Game/ThirdPersonBP/Blueprints/ThirdPersonCharacter` (`GameplayStatics.GetPlayerCharacter` 0) :!pure true)))) (- (.z (.location (`self.GetTransform` (cast `/Game/ThirdPersonBP/Blueprints/ThirdPersonCharacter` (`GameplayStatics.GetPlayerCharacter` 0) :!pure true)))) 98.0)) (.rotation (`self.GetTransform` (cast `/Game/ThirdPersonBP/Blueprints/ThirdPersonCharacter` (`GameplayStatics.GetPlayerCharacter` 0) :!pure true))) (.scale (`self.GetTransform` (cast `/Game/ThirdPersonBP/Blueprints/ThirdPersonCharacter` (`GameplayStatics.GetPlayerCharacter` 0) :!pure true)))))
  (`self.K2_SetActorTransform` _returnvalue)
  (`SceneComponent.K2_SetWorldTransform` (`self.VisualEmitter`) _returnvalue false false))

(fn `UserConstructionScript`)