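; BasicAttack is a telegraphed ability actor that shows a particle warning, then checks for hits once AbilityTime elapses.
; BeginPlay spawns the telegraph emitter and Tick keeps it on the actor's transform at a fixed squashed scale, removing it when the actor is destroyed.
; When the timer expires, overlapping actors other than abilities and the instigator are tested for the Attackable tag, which only prints debug text, and the actor destroys itself.
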(event `self.ReceiveBeginPlay`
  ;[1 1 1] Spawn Effect
  (bind _returnvalue (`GameplayStatics.SpawnEmitterAtLocation` "/Game/Blueprints/Patrick/Abilities/ParticleSystems/TelegraphTwoParticle.TelegraphTwoParticle" (.location (`self.GetTransform`)) (.rotation (`self.GetTransform`)) (.scale (`self.GetTransform`)) false))
  (bind _output_get (set `self.ParticleEffect` _returnvalue))
  (`SceneComponent.SetRelativeScale3D` _output_get (0.5 1.0 1.0))
  (add `self.OnDestroyed` (delegate `OnDestroyed_Event_0`)))

(event `OnDestroyed_Event_0` :!signature `self.OnDestroyed`
  (params (DestroyedActor :type "Actor Object Reference"))
  ;[1 1 1] Spawn Effect
  (`ActorComponent.K2_DestroyComponent` (`self.ParticleEffect`)))

(event `self.ReceiveTick`
  (params (DeltaSeconds :type "Float (single-precision)"))
  ;[1 1 1] Update Effect Transform
  (`SceneComponent.K2_SetWorldTransform` (`self.ParticleEffect`) (`KismetMathLibrary.MakeTransform` (.location (`self.GetTransform`)) (.rotation (`self.GetTransform`)) (0.5 1.0 1.0)) false false)
  (set `self.Timer` (+ (`self.Timer`) DeltaSeconds))
  (if (>= (`self.Timer`) (`self.AbilityTime`))
    ;[1 1 1] Collision hit
    (for _array_element (`self.GetOverlappingActors` "/Script/Engine.Actor")
      (if (`self.ActorHasTag` _array_element "Ability")
        _
        (elif (!= (`self.GetInstigator`) _array_element)
          (if (`self.ActorHasTag` _array_element "Attackable")
            (`KismetSystemLibrary.PrintString` "Damaging Actor")
            (else
              (`KismetSystemLibrary.PrintString` "Actor is not attackable"))))))
    (`self.K2_DestroyActor`)))

(event `self.ReceiveActorBeginOverlap`
  (params (OtherActor :type "Actor Object Reference"))
  ;[1 1 1] Collision hit
)

(fn `UserConstructionScript`)