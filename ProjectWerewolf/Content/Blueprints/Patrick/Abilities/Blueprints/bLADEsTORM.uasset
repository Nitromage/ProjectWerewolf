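; Bladestorm ability actor that follows player 0 at a fixed height and repeatedly damages the actors around them once cast.
; It shows a circle particle until left click casts and sets the cooldown or right click cancels through the player's AbilitySystem.
; While cast, Tick sends mesh overlaps to ServerDamage whenever the timer lands near a DamageInterval multiple, then destroys the actor after CastTime.
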(event `self.ReceiveBeginPlay`
  ;[1 1 1] Spawn Effect
  (bind _returnvalue (`GameplayStatics.SpawnEmitterAtLocation` "/Game/Blueprints/Patrick/Abilities/ParticleSystems/CircleParticle.CircleParticle" (`KismetMathLibrary.MakeVector` (.x (.location (`self.GetTransform`))) (.y (.location (`self.GetTransform`))) 101.0) (.rotation (`self.GetTransform`)) (.scale (`self.GetTransform`)) false))
  (set `self.VisualEmitter` _returnvalue))

(event `Key|LeftMouseButton`
  (params (Key :type "Key Structure"))
  ;[1 1 1] Cancel / Cast
  (:`Pressed`
    (`/Game/Blueprints/Patrick/Abilities/Blueprints/AbilitySystem.SetCooldown` (`/Game/ThirdPersonBP/Blueprints/ThirdPersonCharacter.AbilitySystem` (cast `/Game/ThirdPersonBP/Blueprints/ThirdPersonCharacter` (`GameplayStatics.GetPlayerCharacter` 0) :!pure true)) (`self.Cooldown`))
    (set `self.IsCasted?` true)
    (`self.CleanUp` :!label _label)))

(event `Key|RightMouseButton`
  (params (Key :type "Key Structure"))
  ;[1 1 1] Cancel / Cast
  (:`Pressed`
    (`/Game/Blueprints/Patrick/Abilities/Blueprints/AbilitySystem.CancelAbility` (`/Game/ThirdPersonBP/Blueprints/ThirdPersonCharacter.AbilitySystem` (cast `/Game/ThirdPersonBP/Blueprints/ThirdPersonCharacter` (`GameplayStatics.GetPlayerCharacter` 0) :!pure true)))
    (goto _label)))

(event `self.ReceiveTick`
  (params (DeltaSeconds :type "Float (single-precision)"))
  (bind _asthird_person_character (cast `/Game/ThirdPersonBP/Blueprints/ThirdPersonCharacter` (`GameplayStatics.GetPlayerCharacter` 0) :!pure true))
  ;[1 1 1] Update
  (if (`self.IsCasted?`)
    (`self.UpdatePosition`)
    (bind _output_get (set `self.Timer` (+ (`self.Timer`) DeltaSeconds)))
    (if (<= _output_get (`self.CastTime`))
      (bind _returnvalue (mod _output_get (`self.DamageInterval`)))
      (if (and (> _returnvalue -0.01) (< _returnvalue 0.01))
        (`/Game/Blueprints/Patrick/Abilities/Blueprints/AbilitySystem.Server_damage` (`/Game/ThirdPersonBP/Blueprints/ThirdPersonCharacter.AbilitySystem` _asthird_person_character) _asthird_person_character (`PrimitiveComponent.GetOverlappingActors` (`self.StaticMesh`) "/Script/Engine.Actor") (`self.Damage`)))
      (else
        (`self.K2_DestroyActor`)))
    (else
      (`self.UpdatePosition`))))

(fn `CleanUp`
  (`ActorComponent.K2_DestroyComponent` (`self.VisualEmitter`)))

(fn `MaxLocation`
  (params (PointOne :type "Vector Structure") (PointTwo :type "Vector Structure"))
  (returns (NewPosition :type "Vector Structure"))
  (return (`KismetMathLibrary.MakeVector` (.x (* (`KismetMathLibrary.Normal` (- PointOne PointTwo)) 0.0)) (.y (* (`KismetMathLibrary.Normal` (- PointOne PointTwo)) 0.0)) (+ (.z (* (`KismetMathLibrary.Normal` (- PointOne PointTwo)) 0.0)) 1.0))))

(fn `UpdatePosition`
  (bind _returnvalue (`KismetMathLibrary.MakeTransform` (`KismetMathLibrary.MakeVector` (.x (.location (`self.GetTransform` (cast `/Game/ThirdPersonBP/Blueprints/ThirdPersonCharacter` (`GameplayStatics.GetPlayerCharacter` 0) :!pure true)))) (.y (.location (`self.GetTransform` (cast `/Game/ThirdPersonBP/Blueprints/ThirdPersonCharacter` (`GameplayStatics.GetPlayerCharacter` 0) :!pure true)))) 101.0) (.rotation (`self.GetTransform` (cast `/Game/ThirdPersonBP/Blueprints/ThirdPersonCharacter` (`GameplayStatics.GetPlayerCharacter` 0) :!pure true))) (.scale (`self.GetTransform` (cast `/Game/ThirdPersonBP/Blueprints/ThirdPersonCharacter` (`GameplayStatics.GetPlayerCharacter` 0) :!pure true)))))
  (`self.K2_SetActorTransform` _returnvalue)
  (if (`KismetSystemLibrary.IsValid` (`self.VisualEmitter`))
    (`SceneComponent.K2_SetWorldTransform` (`self.VisualEmitter`) _returnvalue false false)))

(fn `UserConstructionScript`)