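; Spear jump ability actor that shows a ground-target marker, then launches the player at it for an area-damage landing.
; Until cast, a camera-direction trace moves the marker over Landscape, with MaxLocation handling out-of-range hits; right click cancels.
; Left click locks input, starts cooldown and calls SpearLaunch.
; Tick raises gravity above the target for a slam, then on landing restores it, sends effect and overlap damage through AbilitySystem and self-destroys.
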(event `self.ReceiveBeginPlay`
  ;[1 1 1] Spawn Effect
  (bind _returnvalue (`GameplayStatics.SpawnEmitterAtLocation` "/Game/Blueprints/Patrick/Abilities/ParticleSystems/CircleParticle.CircleParticle" (.location (`self.GetTransform`)) (.rotation (`self.GetTransform`)) (.scale (`self.GetTransform`)) false))
  (set `self.VisualEmitter` _returnvalue))

(event `Key|LeftMouseButton`
  (params (Key :type "Key Structure"))
  (bind _asthird_person_character (cast `/Game/ThirdPersonBP/Blueprints/ThirdPersonCharacter` (`GameplayStatics.GetPlayerCharacter` 0) :!pure true))
  ;[1 1 1] Cancel / Cast
  (:`Pressed`
    (`self.CleanUp`)
    (set `self.IsCasted?` true)
    (`self.DisableInput` _asthird_person_character null)
    (set `MovementComponent.Velocity` (0.0 0.0 0.0) (`Pawn.GetMovementComponent` _asthird_person_character))
    (`/Game/Blueprints/Patrick/Abilities/Blueprints/AbilitySystem.SetCooldown` (`/Game/ThirdPersonBP/Blueprints/ThirdPersonCharacter.AbilitySystem` _asthird_person_character) (`self.Cooldown`))
    (`/Game/ThirdPersonBP/Blueprints/ThirdPersonCharacter.SpearLaunch` _asthird_person_character (`self.K2_GetActorLocation`))))

(event `Key|RightMouseButton`
  (params (Key :type "Key Structure"))
  ;[1 1 1] Cancel / Cast
  (:`Pressed`
    (`/Game/Blueprints/Patrick/Abilities/Blueprints/AbilitySystem.CancelAbility` (`/Game/ThirdPersonBP/Blueprints/ThirdPersonCharacter.AbilitySystem` (cast `/Game/ThirdPersonBP/Blueprints/ThirdPersonCharacter` (`GameplayStatics.GetPlayerCharacter` 0) :!pure true)))
    (`self.CleanUp`)
    (`self.K2_DestroyActor`)))

(event `self.ReceiveTick`
  (params (DeltaSeconds :type "Float (single-precision)"))
  (bind _asthird_person_character (cast `/Game/ThirdPersonBP/Blueprints/ThirdPersonCharacter` (`GameplayStatics.GetPlayerCharacter` 0) :!pure true))
  (bind _abilitysystem (`/Game/ThirdPersonBP/Blueprints/ThirdPersonCharacter.AbilitySystem` _asthird_person_character))
  ;[1 1 1] Update
  (if (`self.IsCasted?`)
    (if (`KismetMathLibrary.NearlyEqual_TransformTransform` (`KismetMathLibrary.MakeTransform` (`KismetMathLibrary.MakeVector` (.x (`self.K2_GetActorLocation` _asthird_person_character)) (.y (`self.K2_GetActorLocation` _asthird_person_character)))) (`KismetMathLibrary.MakeTransform` (`KismetMathLibrary.MakeVector` (.x (`self.K2_GetActorLocation`)) (.y (`self.K2_GetActorLocation`)))) 100.0)
      (`KismetSystemLibrary.Delay` 0.2)
      (`/Game/ThirdPersonBP/Blueprints/ThirdPersonCharacter.Gravity` _asthird_person_character 100.0)
      (else
        (`KismetSystemLibrary.Delay` 0.2)))
    (if (not (`NavMovementComponent.IsFalling` (`Character.CharacterMovement` _asthird_person_character)))
      (`/Game/ThirdPersonBP/Blueprints/ThirdPersonCharacter.Gravity` _asthird_person_character 1.0)
      (if (not (`self.Spawned`))
        (set `self.Spawned` true)
        (`/Game/Blueprints/Patrick/Abilities/Blueprints/AbilitySystem.Server_Cast` _abilitysystem (`self.GetTransform`) (`|MakeArray` "/Game/Blueprints/Patrick/Abilities/ParticleSystems/SpearJump.SpearJump" :!type "ParticleSystem Object Reference")))
      (`/Game/Blueprints/Patrick/Abilities/Blueprints/AbilitySystem.Server_damage` _abilitysystem _asthird_person_character (`PrimitiveComponent.GetOverlappingActors` (`self.StaticMesh`) "/Script/Engine.Actor") (`self.Damage`))
      (`self.EnableInput` _asthird_person_character null)
      (`self.K2_DestroyActor`))
    (else
      (`self.UpdatePosition`))))

(fn `CleanUp`
  (`ActorComponent.K2_DestroyComponent` (`self.VisualEmitter`)))

(fn `MaxLocation`
  (params (PointOne :type "Vector Structure") (PointTwo :type "Vector Structure"))
  (returns (NewPosition :type "Vector Structure"))
  (return (`KismetMathLibrary.MakeVector` (.x (* (`KismetMathLibrary.Normal` (- PointOne PointTwo)) (`self.AbilityRange`))) (.y (* (`KismetMathLibrary.Normal` (- PointOne PointTwo)) (`self.AbilityRange`))) (+ (.z (* (`KismetMathLibrary.Normal` (- PointOne PointTwo)) (`self.AbilityRange`))) 1.0))))

(fn `UpdatePosition`
  (bind _returnvalue (`self.GetActorScale3D`))
  (bind _asthird_person_character (cast `/Game/ThirdPersonBP/Blueprints/ThirdPersonCharacter` (`GameplayStatics.GetPlayerCharacter` 0)))
  (bind _returnvalue_2 (`self.K2_GetActorLocation` _asthird_person_character))
  (bind _outhit (`KismetSystemLibrary.LineTraceSingle` _returnvalue_2 (+ _returnvalue_2 (* (`KismetMathLibrary.GetForwardVector` (`Pawn.GetControlRotation` _asthird_person_character)) 5000.0)) "TraceTypeQuery1"))
  (bind (_bblockinghit _binitialoverlap _time _distance _location _impactpoint _normal _impactnormal _physmat _hitactor) (`GameplayStatics.BreakHitResult` _outhit))
  (if _bblockinghit
    (if (> _distance (`self.AbilityRange`))
      ;[1 1 1] Max cast range
      (bind _newposition (`self.MaxLocation` (.location (`self.GetTransform` (cast `/Game/ThirdPersonBP/Blueprints/ThirdPersonCharacter` (`GameplayStatics.GetPlayerCharacter` 0) :!pure true))) _location))
      (bind _returnvalue_3 (`KismetMathLibrary.MakeRotFromZ` _normal))
      (bind _returnvalue_4 (`KismetMathLibrary.MakeTransform` _newposition _returnvalue_3 _returnvalue))
      (`self.K2_SetActorTransform` _returnvalue_4)
      (`SceneComponent.K2_SetWorldTransform` (`self.VisualEmitter`) _returnvalue_4 false false)
      (else
        (cast `Landscape` _hitactor)
        (bind _returnvalue_5 (`KismetMathLibrary.MakeTransform` (`KismetMathLibrary.MakeVector` (.x _location) (.y _location) (+ (.z _location) 1.0)) _returnvalue_3 _returnvalue))
        (`self.K2_SetActorTransform` _returnvalue_5)
        (`SceneComponent.K2_SetWorldTransform` (`self.VisualEmitter`) _returnvalue_5 false false)))))

(fn `UserConstructionScript`)