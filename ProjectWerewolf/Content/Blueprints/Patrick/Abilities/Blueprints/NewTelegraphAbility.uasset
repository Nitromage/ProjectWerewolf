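; Telegraphed attack ability actor that fills a warning indicator over a charge time, then strikes everything overlapping it.
; Tick advances a timer that drives the Fill parameter of a dynamic material.
; At full charge, it skips the instigator and Ability-tagged actors, grants the instigator wood for trees and deals the instigator's damage to structures and characters.
; It then re-enables attacking on player character 0 and destroys itself.
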(event `self.ReceiveBeginPlay`
  (bind _returnvalue (`self.GetInstigator`))
  (bind _asthird_person_character (cast `/Game/ThirdPersonBP/Blueprints/ThirdPersonCharacter` _returnvalue :!pure true))
  (bind _damage (`/Game/ThirdPersonBP/Blueprints/ThirdPersonCharacter.Damage` _asthird_person_character))
  ;[1 1 1] Setup fill
  (bind _returnvalue_2 (`PrimitiveComponent.CreateDynamicMaterialInstance` (`self.Fill`) 0 "/Game/Blueprints/Patrick/Abilities/Materials/NewTelegraphMat.NewTelegraphMat"))
  (set `self.ProgressBarMat` _returnvalue_2)
  (`MaterialInstanceDynamic.SetScalarParameterValue` (`self.ProgressBarMat`) "Fill" (`self.FillAmount`) :!label _label)
  (if (>= (stale `self.ReceiveTick` _output_get_2) 1.0)
    ;[1 1 1] Collision hit
    (for _array_element (`self.GetOverlappingActors` "/Script/Engine.Actor")
      (if (`self.ActorHasTag` _array_element "Ability")
        _
        (elif (!= _returnvalue _array_element)
          (if (`self.ActorHasTag` _array_element "Tree")
            (`/Game/ThirdPersonBP/Blueprints/ThirdPersonCharacter.Wood` _asthird_person_character 5 true)
            (else
              (bind _asstructure (cast `/Game/Blueprints/Patrick/Buildings/Structure` _array_element)
                (:`then`
                  (`GameplayStatics.ApplyDamage` _asstructure _damage null null "/Script/Engine.DamageType"))
                (:`CastFailed`
                  (bind _asthird_person_character_2 (cast `/Game/ThirdPersonBP/Blueprints/ThirdPersonCharacter` _array_element))
                  (`GameplayStatics.ApplyDamage` _asthird_person_character_2 _damage null null "/Script/Engine.DamageType"))))))))
    (`self.OnClient`)
    (`self.K2_DestroyActor`)))

(event `self.ReceiveTick`
  (params (DeltaSeconds :type "Float (single-precision)"))
  ;[1 1 1] Update fill
  (bind _output_get (set `self.Timer` (+ (`self.Timer`) DeltaSeconds)))
  (bind _output_get_2 (set `self.FillAmount` (/ _output_get (`self.ChargeTime`))))
  (goto _label))

(event `OnClient`
  (bind _asthird_person_character (cast `/Game/ThirdPersonBP/Blueprints/ThirdPersonCharacter` (`GameplayStatics.GetPlayerCharacter` 0)))
  (set `/Game/ThirdPersonBP/Blueprints/ThirdPersonCharacter.CanAttack?` true _asthird_person_character))

(fn `UserConstructionScript`)