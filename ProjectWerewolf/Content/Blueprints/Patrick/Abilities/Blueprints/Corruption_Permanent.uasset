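; Permanent corruption zone ability that spawns a Corruption particle effect and spreads outward with no built-in limit or expiry.
; Structures and trees that begin overlapping it get flagged as corrupted.
; A Tick timer widens both actor and emitter in X and Y at a fixed interval.
; Each interval first runs TickDamage, which damages overlapping ThirdPersonCharacters and Structures, but not trees.
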(event `self.ReceiveBeginPlay`
  (bind _returnvalue (`GameplayStatics.SpawnEmitterAtLocation` "/Game/Blueprints/Patrick/Abilities/ParticleSystems/Corruption.Corruption" (.location (`self.GetTransform`)) (.rotation (`self.GetTransform`)) (.scale (`self.GetTransform`))))
  (set `self.Emitter` _returnvalue))

(event `self.ReceiveActorBeginOverlap`
  (params (OtherActor :type "Actor Object Reference"))
  (bind _asstructure (cast `/Game/Blueprints/Patrick/Buildings/Structure` OtherActor)
    (:`then`
      (set `/Game/Blueprints/Patrick/Buildings/Structure.IsCorrupted?` true _asstructure))
    (:`CastFailed`
      (bind _astree (cast `/Game/Blueprints/Patrick/Tree` OtherActor))
      (set `/Game/Blueprints/Patrick/Tree.IsCorrupted?` true _astree))))

(event `self.ReceiveTick`
  (params (DeltaSeconds :type "Float (single-precision)"))
  (bind _enlargeby (`self.EnlargeBy`))
  (bind _returnvalue (`KismetMathLibrary.MakeTransform` (.location (`self.GetTransform`)) (.rotation (`self.GetTransform`)) (`KismetMathLibrary.MakeVector` (+ (.x (.scale (`self.GetTransform`))) _enlargeby) (+ (.y (.scale (`self.GetTransform`))) _enlargeby) (.z (.scale (`self.GetTransform`))))))
  (bind _output_get (set `self.Timer` (+ (`self.Timer`) DeltaSeconds)))
  (if (>= _output_get (`self.EnlargeTime`))
    (set `self.Timer` 0.0)
    (`self.TickDamage`)
    (`SceneComponent.K2_SetWorldTransform` (`self.Emitter`) _returnvalue false false)
    (`self.K2_SetActorTransform` _returnvalue)))

(fn `TickDamage`
  (bind _damage (`self.Damage`))
  (for _array_element (`self.GetOverlappingActors` "/Script/Engine.Actor")
    (bind _asthird_person_character (cast `/Game/ThirdPersonBP/Blueprints/ThirdPersonCharacter` _array_element)
      (:`then`
        (`GameplayStatics.ApplyDamage` _asthird_person_character _damage))
      (:`CastFailed`
        (bind _asstructure (cast `/Game/Blueprints/Patrick/Buildings/Structure` _array_element))
        (`GameplayStatics.ApplyDamage` _asstructure _damage)))))

(fn `UserConstructionScript`)