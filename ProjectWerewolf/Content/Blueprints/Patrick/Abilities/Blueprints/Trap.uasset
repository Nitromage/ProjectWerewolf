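; Trap ability actor that acts as both the caster and the placed trap, switched by IsCasted.
; On BeginPlay it sets player 0's cooldown and disables input; after a short delay, an uncast instance calls ServerTrap at the player's position with fixed height, self-destructs and re-enables input.
; A cast trap damages and stuns the first overlapping non-User actor through player 0's AbilitySystem, then destroys itself, or expires after LifeTime.
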(event `self.ReceiveBeginPlay`
  (bind _asthird_person_character (cast `/Game/ThirdPersonBP/Blueprints/ThirdPersonCharacter` (`GameplayStatics.GetPlayerCharacter` 0) :!pure true))
  (bind _abilitysystem (`/Game/ThirdPersonBP/Blueprints/ThirdPersonCharacter.AbilitySystem` _asthird_person_character))
  (`/Game/Blueprints/Patrick/Abilities/Blueprints/AbilitySystem.SetCooldown` _abilitysystem (`self.Cooldown`))
  (`self.DisableInput` _asthird_person_character null)
  (`KismetSystemLibrary.Delay` 0.2)
  (if (not (`self.IsCasted?`))
    (`/Game/Blueprints/Patrick/Abilities/Blueprints/AbilitySystem.Server_Trap` _abilitysystem (`KismetMathLibrary.MakeTransform` (`KismetMathLibrary.MakeVector` (.x (.location (`self.GetTransform` _asthird_person_character))) (.y (.location (`self.GetTransform` _asthird_person_character))) 100.0) (.rotation (`self.GetTransform` _asthird_person_character)) (.scale (`self.GetTransform` _asthird_person_character))) _asthird_person_character)
    (`self.K2_DestroyActor`)
    (`self.EnableInput` _asthird_person_character null)))

(event `self.ReceiveActorBeginOverlap`
  (params (OtherActor :type "Actor Object Reference"))
  (bind _array (`|MakeArray` OtherActor))
  (bind _user (`self.User`))
  (bind _abilitysystem (`/Game/ThirdPersonBP/Blueprints/ThirdPersonCharacter.AbilitySystem` (cast `/Game/ThirdPersonBP/Blueprints/ThirdPersonCharacter` (`GameplayStatics.GetPlayerCharacter` 0) :!pure true)))
  (if (`self.IsCasted?`)
    (if (!= _user OtherActor)
      (`/Game/Blueprints/Patrick/Abilities/Blueprints/AbilitySystem.Server_damage` _abilitysystem _user _array (`self.Damage`))
      (`/Game/Blueprints/Patrick/Abilities/Blueprints/AbilitySystem.Server_Stun` _abilitysystem null _array (`self.StunTime`))
      (`self.K2_DestroyActor`))))

(event `self.ReceiveTick`
  (params (DeltaSeconds :type "Float (single-precision)"))
  (if (`self.IsCasted?`)
    (bind _output_get (set `self.Timer` (+ (`self.Timer`) DeltaSeconds)))
    (if (>= _output_get (`self.LifeTime`))
      (`self.K2_DestroyActor`))))

(fn `UserConstructionScript`)