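; GrabAttack is an aimed charge ability actor that stuns and damages characters it hits.
; Before casting, it holds an arrow emitter in front of player 0; right click cancels.
; Left click while grounded removes the arrow, sets cooldown and calls ServerCharge.
; The actor keeps following as a hitbox, applying effects through the player's AbilitySystem on overlap, then zeroes velocity and destroys itself after a short delay.
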(event `self.ReceiveBeginPlay`
  ;[1 1 1] Spawn Effect
  (bind _returnvalue (`GameplayStatics.SpawnEmitterAtLocation` "/Game/Blueprints/Patrick/Abilities/ParticleSystems/Arrow.Arrow" (.location (`self.GetTransform`)) (.rotation (`self.GetTransform`)) (.scale (`self.GetTransform`)) false))
  (set `self.VisualEmitter` _returnvalue))

(event `Key|LeftMouseButton`
  (params (Key :type "Key Structure"))
  (bind _asthird_person_character (cast `/Game/ThirdPersonBP/Blueprints/ThirdPersonCharacter` (`GameplayStatics.GetPlayerCharacter` 0) :!pure true))
  (:`Pressed`
    ;[1 1 1] Cancel / Cast
    (if (`NavMovementComponent.IsMovingOnGround` (`Character.CharacterMovement` (cast `/Game/ThirdPersonBP/Blueprints/ThirdPersonCharacter` (`GameplayStatics.GetPlayerCharacter` 0) :!pure true)))
      (`self.CleanUp`)
      (set `self.IsCasted?` true)
      (`/Game/Blueprints/Patrick/Abilities/Blueprints/AbilitySystem.SetCooldown` (`/Game/ThirdPersonBP/Blueprints/ThirdPersonCharacter.AbilitySystem` _asthird_person_character) (`self.Cooldown`))
      (`/Game/ThirdPersonBP/Blueprints/ThirdPersonCharacter.ServerCharge` _asthird_person_character (`self.ChargeLength`)))))

(event `Key|RightMouseButton`
  (params (Key :type "Key Structure"))
  ;[1 1 1] Cancel / Cast
  (:`Pressed`
    (`/Game/Blueprints/Patrick/Abilities/Blueprints/AbilitySystem.CancelAbility` (`/Game/ThirdPersonBP/Blueprints/ThirdPersonCharacter.AbilitySystem` (cast `/Game/ThirdPersonBP/Blueprints/ThirdPersonCharacter` (`GameplayStatics.GetPlayerCharacter` 0) :!pure true)))
    (`self.CleanUp`)
    (`self.K2_DestroyActor`)))

(event `self.ReceiveActorBeginOverlap`
  (params (OtherActor :type "Actor Object Reference"))
  (bind _asthird_person_character (cast `/Game/ThirdPersonBP/Blueprints/ThirdPersonCharacter` (`GameplayStatics.GetPlayerCharacter` 0) :!pure true))
  (bind _abilitysystem (`/Game/ThirdPersonBP/Blueprints/ThirdPersonCharacter.AbilitySystem` _asthird_person_character))
  (if (`self.IsCasted?`)
    (bind _asthird_person_character_2 (cast `/Game/ThirdPersonBP/Blueprints/ThirdPersonCharacter` OtherActor))
    (bind _array (`|MakeArray` _asthird_person_character_2 :!type "Actor Object Reference"))
    (`/Game/Blueprints/Patrick/Abilities/Blueprints/AbilitySystem.Server_Stun` _abilitysystem _asthird_person_character _array (`self.StunTime`))
    (`/Game/Blueprints/Patrick/Abilities/Blueprints/AbilitySystem.Server_damage` _abilitysystem _asthird_person_character _array (`self.Damage`))
    (set `MovementComponent.Velocity` (0.0 0.0 0.0) (`Pawn.GetMovementComponent` _asthird_person_character))))

(event `self.ReceiveTick`
  (params (DeltaSeconds :type "Float (single-precision)"))
  (bind _charactermovement (`Character.CharacterMovement` (cast `/Game/ThirdPersonBP/Blueprints/ThirdPersonCharacter` (`GameplayStatics.GetPlayerCharacter` 0) :!pure true)))
  ;[1 1 1] Update
  (if (`self.IsCasted?`)
    (if (not (`NavMovementComponent.IsMovingOnGround` _charactermovement))
      (set `MovementComponent.Velocity` (0.0 0.0 0.0) _charactermovement))
    (`self.UpdatePosition`)
    (`KismetSystemLibrary.Delay` 0.2)
    (set `MovementComponent.Velocity` (0.0 0.0 0.0) _charactermovement)
    (`self.K2_DestroyActor`)
    (else
      (`self.UpdatePosition`))))

(fn `CleanUp`
  (`ActorComponent.K2_DestroyComponent` (`self.VisualEmitter`)))

(fn `MaxLocation`
  (params (PointOne :type "Vector Structure") (PointTwo :type "Vector Structure"))
  (returns (NewPosition :type "Vector Structure"))
  (return (`KismetMathLibrary.MakeVector` (.x (* (`KismetMathLibrary.Normal` (- PointOne PointTwo)) (`self.AbilityRange`))) (.y (* (`KismetMathLibrary.Normal` (- PointOne PointTwo)) (`self.AbilityRange`))) (+ (.z (* (`KismetMathLibrary.Normal` (- PointOne PointTwo)) (`self.AbilityRange`))) 1.0))))

(fn `UpdatePosition`
  (bind _asthird_person_character (cast `/Game/ThirdPersonBP/Blueprints/ThirdPersonCharacter` (`GameplayStatics.GetPlayerCharacter` 0) :!pure true))
  (bind _returnvalue (`KismetMathLibrary.MakeTransform` (`KismetMathLibrary.MakeVector` (.x (+ (* (`KismetMathLibrary.Normal` (`self.GetActorForwardVector` _asthird_person_character)) 200) (.location (`self.GetTransform` _asthird_person_character)))) (.y (+ (* (`KismetMathLibrary.Normal` (`self.GetActorForwardVector` _asthird_person_character)) 200) (.location (`self.GetTransform` _asthird_person_character)))) 101.0) (`KismetMathLibrary.MakeRotator` (.roll (.rotation (`self.GetTransform` _asthird_person_character))) (.pitch (.rotation (`self.GetTransform` _asthird_person_character))) (+ (.yaw (.rotation (`self.GetTransform` _asthird_person_character))) 180.0)) (1.5 1.5 1.0)))
  (`self.K2_SetActorTransform` _returnvalue)
  (if (not (`self.IsCasted?`))
    (`SceneComponent.K2_SetWorldTransform` (`self.VisualEmitter`) _returnvalue false false)))

(fn `UserConstructionScript`)