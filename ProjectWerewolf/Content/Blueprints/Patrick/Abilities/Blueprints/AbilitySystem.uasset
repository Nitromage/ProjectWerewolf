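; Ability component for a ThirdPersonCharacter that spawns and aims telegraphed attacks and plays melee montages.
; SpawnOnServer calls BasicAttack to spawn a telegraph box, which Tick keeps ahead of the owner along control yaw at fixed height.
; AbilityOne line-traces along control rotation and spawns its ability actor aligned to the surface normal, only on Landscape hits.
; PunchAnimation picks a montage by character subclass and, for Kachu, by weapon.
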(event `self.ReceiveTick`
  (params (DeltaSeconds :type "Float (single-precision)"))
  (bind _abilitybox (`self.AbilityBox`))
  (bind _abilitybox_2 (`self.AbilityBox`))
  ;[1 1 1] Update Basic Attack
  (if (`KismetSystemLibrary.IsValid` _abilitybox_2)
    (bind _asnew_telegraph_ability (cast `/Game/Blueprints/Patrick/Abilities/Blueprints/NewTelegraphAbility` _abilitybox_2))
    (bind _transform (`self.GetFrontTransform` (`/Game/Blueprints/Patrick/Abilities/Blueprints/NewTelegraphAbility.DistanceFromPlayer` _asnew_telegraph_ability)))
    (bind _asnew_telegraph_ability_2 (cast `/Game/Blueprints/Patrick/Abilities/Blueprints/NewTelegraphAbility` _abilitybox)
      (:`then`
        (`Actor.K2_SetActorTransform` _asnew_telegraph_ability_2 (`KismetMathLibrary.MakeTransform` (.location _transform) (.rotation _transform) (`/Game/Blueprints/Patrick/Abilities/Blueprints/NewTelegraphAbility.Scale` _asnew_telegraph_ability_2)) false false))
      (:`CastFailed`
        (`Actor.K2_SetActorTransform` _abilitybox _transform false false)))))

(event `SpawnOnServer`
  (bind (_animationtime _abilitybox) (`self.BasicAttack`))
  (set `self.AbilityBox` _abilitybox))

(fn `AbilityOne`
  (locals (Range :type "Float (double-precision)" :default 1000.0))
  (bind _asthird_person_character (cast `/Game/ThirdPersonBP/Blueprints/ThirdPersonCharacter` (`self.GetOwner`)))
  (bind _returnvalue (`Actor.K2_GetActorLocation` _asthird_person_character))
  (bind _outhit (`KismetSystemLibrary.LineTraceSingle` _returnvalue (+ _returnvalue (* (`KismetMathLibrary.GetForwardVector` (`Pawn.GetControlRotation` _asthird_person_character)) (`local.Range`))) "TraceTypeQuery1"))
  (bind (_bblockinghit _binitialoverlap _time _distance _location _impactpoint _normal _impactnormal _physmat _hitactor) (`GameplayStatics.BreakHitResult` _outhit))
  (if _bblockinghit
    (cast `Landscape` _hitactor)
    (bind _returnvalue_2 (`|SpawnActorFromClass` "/Game/Blueprints/Patrick/Abilities/Blueprints/AbilityOne.AbilityOne_C" (`KismetMathLibrary.MakeTransform` (`KismetMathLibrary.MakeVector` (.x _location) (.y _location) (+ (.z _location) 1.0)) (`KismetMathLibrary.MakeRotFromZ` _normal)) "Undefined" "OverrideRootScale" null _asthird_person_character))
    (set `/Game/Blueprints/Patrick/Abilities/Blueprints/AbilityOne.Range` (`local.Range`) _returnvalue_2)
    (set `self.CurrentAbility` _returnvalue_2)))

(fn `BasicAttack`
  (returns (AnimationTime :type "Float (double-precision)") (AbilityBox :type "Actor Object Reference"))
  (bind _returnvalue (`self.GetOwner`))
  (bind _asthird_person_character (cast `/Game/ThirdPersonBP/Blueprints/ThirdPersonCharacter` (`self.GetOwner`)))
  (bind _asthird_person_character_2 (cast `/Game/ThirdPersonBP/Blueprints/ThirdPersonCharacter` _returnvalue))
  (bind _returnvalue_2 (`KismetMathLibrary.GetForwardVector` (`KismetMathLibrary.MakeRotator` 0.0 0.0 (.yaw (`Pawn.GetControlRotation` _asthird_person_character)))))
  (bind _returnvalue_3 (`|SpawnActorFromClass` "/Game/Blueprints/Patrick/Abilities/Blueprints/NewTelegraphAbility.NewTelegraphAbility_C" (`KismetMathLibrary.MakeTransform` (`KismetMathLibrary.MakeVector` (.x (+ (.location (`Actor.GetTransform` _returnvalue)) (* _returnvalue_2 150.0))) (.y (+ (.location (`Actor.GetTransform` _returnvalue)) (* _returnvalue_2 150.0))) 101.0) (`KismetMathLibrary.MakeRotator` (.roll (.rotation (`Actor.GetTransform` _returnvalue))) (.pitch (.rotation (`Actor.GetTransform` _returnvalue))) (+ (.yaw (`KismetMathLibrary.MakeRotFromZ` _returnvalue_2)) 90.0)) (.scale (`Actor.GetTransform` _returnvalue))) "Undefined" "OverrideRootScale" null _asthird_person_character_2))
  (set `self.AbilityBox` _returnvalue_3)
  (return 2.0 _returnvalue_3))

(fn `GetFrontTransform`
  (params (Distance :type "Float (double-precision)"))
  (returns (Transform :type "Transform Structure"))
  (bind _asthird_person_character (cast `/Game/ThirdPersonBP/Blueprints/ThirdPersonCharacter` (`self.GetOwner`)))
  (bind _returnvalue (`KismetMathLibrary.GetForwardVector` (`KismetMathLibrary.MakeRotator` 0.0 0.0 (.yaw (`Pawn.GetControlRotation` _asthird_person_character)))))
  (return (`KismetMathLibrary.MakeTransform` (`KismetMathLibrary.MakeVector` (.x (+ (.location (`Actor.GetTransform` (`self.GetOwner`))) (* _returnvalue Distance))) (.y (+ (.location (`Actor.GetTransform` (`self.GetOwner`))) (* _returnvalue Distance))) 101.0) (`KismetMathLibrary.MakeRotator` (.roll (.rotation (`Actor.GetTransform` (`self.GetOwner`)))) (.pitch (.rotation (`Actor.GetTransform` (`self.GetOwner`)))) (+ (.yaw (`KismetMathLibrary.MakeRotFromZ` _returnvalue)) 90.0)) (0.4 1.0 1.0))))

(fn `PunchAnimation`
  (bind _returnvalue (`self.GetOwner`))
  (bind _asarcher (cast `/Game/ThirdPersonBP/Blueprints/Archer` _returnvalue)
    (:`then`
      (`Character.PlayAnimMontage` _asarcher "/Game/Blueprints/Steffen/Charatcers/Arissa/Animations/APunchMontage.APunchMontage" 1.0 "None"))
    (:`CastFailed`
      (bind _askachu (cast `/Game/ThirdPersonBP/Blueprints/Kachu` _returnvalue)
        (:`then`
          (if (`/Game/ThirdPersonBP/Blueprints/Kachu.Sword?` _askachu)
            (`Character.PlayAnimMontage` _askachu "/Game/Blueprints/Steffen/Charatcers/Kachu/Animations/KSwordAttack.KSwordAttack" 1.0 "None")
            (elif (`/Game/ThirdPersonBP/Blueprints/Kachu.Spear?` _askachu)
              (`Character.PlayAnimMontage` _askachu "/Game/Blueprints/Steffen/Charatcers/Kachu/Animations/KSpearAttack.KSpearAttack" 1.0 "None")
              (else
                (`Character.PlayAnimMontage` _askachu "/Game/Blueprints/Steffen/Charatcers/Kachu/Animations/KPunchMontage.KPunchMontage" 1.0 "None")))))
        (:`CastFailed`
          (bind _aseve (cast `/Game/ThirdPersonBP/Blueprints/Eve` _returnvalue)
            (:`then`
              (`Character.PlayAnimMontage` _aseve "/Game/Blueprints/Steffen/Charatcers/Eve/Animatoins/EPunchMontage.EPunchMontage" 1.0 "None"))
            (:`CastFailed`
              (bind _aszombie (cast `/Game/ThirdPersonBP/Blueprints/Zombie` _returnvalue)
                (:`then`
                  (`Character.PlayAnimMontage` _aszombie "/Game/Blueprints/Steffen/Charatcers/Zombie/Animations/ZPunchMontage.ZPunchMontage" 1.0 "None"))
                (:`CastFailed`
                  (bind _asthird_person_character (cast `/Game/ThirdPersonBP/Blueprints/ThirdPersonCharacter` _returnvalue))
                  (`Character.PlayAnimMontage` _asthird_person_character "/Game/Blueprints/Patrick/Animations/ArcherAnimations/PunchMontage.PunchMontage" 1.0 "None"))))))))))