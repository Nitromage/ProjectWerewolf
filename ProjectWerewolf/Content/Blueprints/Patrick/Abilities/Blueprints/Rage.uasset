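; Rage is an ability actor that raises the player 0 ThirdPersonCharacter's damage.
; BeginPlay applies DamageBoost, casts the Rage emitter through the AbilitySystem's ServerCast and briefly disables input.
; Tick snaps the actor to the character and accumulates a timer against BoostTime.
; As wired, it destroys itself while the timer is below BoostTime, so the damage-removal branch normally never runs.
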(event `self.ReceiveBeginPlay`
  (bind _asthird_person_character (cast `/Game/ThirdPersonBP/Blueprints/ThirdPersonCharacter` (`GameplayStatics.GetPlayerCharacter` 0) :!pure true))
  (`self.DisableInput` _asthird_person_character null)
  (`/Game/ThirdPersonBP/Blueprints/ThirdPersonCharacter.Dmg` _asthird_person_character (`self.DamageBoost`) true)
  (`/Game/Blueprints/Patrick/Abilities/Blueprints/AbilitySystem.Server_Cast` (`/Game/ThirdPersonBP/Blueprints/ThirdPersonCharacter.AbilitySystem` _asthird_person_character) (`self.GetTransform` _asthird_person_character) (`|MakeArray` "/Game/Blueprints/Patrick/Abilities/ParticleSystems/Rage.Rage" :!type "ParticleSystem Object Reference"))
  (`KismetSystemLibrary.Delay` 0.2)
  (`self.EnableInput` _asthird_person_character null))

(event `self.ReceiveTick`
  (params (DeltaSeconds :type "Float (single-precision)"))
  (`self.K2_SetActorTransform` (`self.GetTransform` (cast `/Game/ThirdPersonBP/Blueprints/ThirdPersonCharacter` (`GameplayStatics.GetPlayerCharacter` 0) :!pure true)))
  (bind _output_get (set `self.Timer` (+ (`self.Timer`) DeltaSeconds)))
  (if (>= _output_get (`self.BoostTime`))
    (`/Game/ThirdPersonBP/Blueprints/ThirdPersonCharacter.Dmg` (cast `/Game/ThirdPersonBP/Blueprints/ThirdPersonCharacter` (`GameplayStatics.GetPlayerCharacter` 0) :!pure true) (`self.DamageBoost`) false)
    (else
      (`self.K2_DestroyActor`))))

(fn `UserConstructionScript`)