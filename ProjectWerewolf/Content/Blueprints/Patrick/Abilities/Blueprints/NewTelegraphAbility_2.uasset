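; Telegraphed area-attack ability actor that shows a charge-up fill, then damages what overlaps it and destroys itself.
; BeginPlay creates a dynamic material on the Fill component, and Tick drives its Fill parameter from elapsed time over ChargeTime.
; At full charge it loops over overlapping actors, skipping the instigator and Ability-tagged actors.
; TestDmgOnServer applies fixed damage to those tagged Attackable, reading the loop's current element directly.
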(event `self.ReceiveBeginPlay`
  ;[1 1 1] Setup fill
  (bind _returnvalue (`PrimitiveComponent.CreateDynamicMaterialInstance` (`self.Fill`) 0 "/Game/Blueprints/Patrick/Abilities/Materials/NewTelegraphMat_2.NewTelegraphMat_2"))
  (set `self.ProgressBarMat` _returnvalue)
  (`MaterialInstanceDynamic.SetScalarParameterValue` (`self.ProgressBarMat`) "Fill" (`self.FillAmount`) :!label _label)
  (if (>= (stale `self.ReceiveTick` _output_get_2) 1.0)
    ;[1 1 1] Collision hit
    (for _array_element (`self.GetOverlappingActors` "/Script/Engine.Actor")
      (if (`self.ActorHasTag` _array_element "Ability")
        _
        (elif (!= (`self.GetInstigator`) _array_element)
          (`self.TestDmgOnServer`))))
    (`self.K2_DestroyActor`)))

(event `TestDmgOnServer`
  ;[1 1 1] Collision hit
  (if (`self.ActorHasTag` (stale `self.ReceiveBeginPlay` _array_element) "Attackable")
    (`GameplayStatics.ApplyDamage` (stale `self.ReceiveBeginPlay` _array_element) 200.0)
    (`KismetSystemLibrary.PrintString` "Damaging Actor")
    (else
      (`KismetSystemLibrary.PrintString` "Actor is not attackable"))))

(event `self.ReceiveTick`
  (params (DeltaSeconds :type "Float (single-precision)"))
  ;[1 1 1] Update fill
  (bind _output_get (set `self.Timer` (+ (`self.Timer`) DeltaSeconds)))
  (bind _output_get_2 (set `self.FillAmount` (/ _output_get (`self.ChargeTime`))))
  (goto _label))

(fn `UserConstructionScript`)