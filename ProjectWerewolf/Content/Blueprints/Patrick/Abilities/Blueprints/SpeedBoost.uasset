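; Speed boost ability actor that temporarily raises the movement speed of player character 0.
; BeginPlay caches the mesh's first material and applies the boost, while Tick keeps the actor at the character, slightly offset along the control rotation.
; During CastTime, Tick sets a green leaf material through the AbilitySystem's MatServer, with a delayed revert.
; On expiry it restores the material, removes the boost and destroys itself.
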(event `self.ReceiveBeginPlay`
  (bind _asthird_person_character (cast `/Game/ThirdPersonBP/Blueprints/ThirdPersonCharacter` (`GameplayStatics.GetPlayerCharacter` 0) :!pure true))
  ;[1 1 1] Spawn Effect
  (set `self.Material` (`PrimitiveComponent.GetMaterial` (`Character.Mesh` _asthird_person_character) 0))
  (`/Game/ThirdPersonBP/Blueprints/ThirdPersonCharacter.Speed` _asthird_person_character 500.0 true))

(event `self.ReceiveTick`
  (params (DeltaSeconds :type "Float (single-precision)"))
  (bind _asthird_person_character (cast `/Game/ThirdPersonBP/Blueprints/ThirdPersonCharacter` (`GameplayStatics.GetPlayerCharacter` 0) :!pure true))
  (bind _mesh (`Character.Mesh` _asthird_person_character))
  (bind _abilitysystem (`/Game/ThirdPersonBP/Blueprints/ThirdPersonCharacter.AbilitySystem` _asthird_person_character))
  ;[1 1 1] Update
  (`self.UpdatePosition`)
  (bind _output_get (set `self.Timer` (+ (`self.Timer`) DeltaSeconds)))
  (if (<= _output_get (`self.CastTime`))
    (`/Game/Blueprints/Patrick/Abilities/Blueprints/AbilitySystem.MatServer` _abilitysystem _mesh 0 "/Game/Shared_Assets/LowPolyAssets/Foliage/Bushes/Materials/Leafs_Green_13.Leafs_Green_13")
    (`KismetSystemLibrary.Delay` 0.5)
    (`/Game/Blueprints/Patrick/Abilities/Blueprints/AbilitySystem.MatServer` _abilitysystem _mesh 0 (`self.Material`))
    (else
      (`/Game/Blueprints/Patrick/Abilities/Blueprints/AbilitySystem.MatServer` _abilitysystem _mesh 0 (`self.Material`))
      (`/Game/ThirdPersonBP/Blueprints/ThirdPersonCharacter.Speed` _asthird_person_character 500.0 false)
      (`self.K2_DestroyActor`))))

(fn `CleanUp`
  (`ActorComponent.K2_DestroyComponent` (`self.VisualEmitter`)))

(fn `MaxLocation`
  (params (PointOne :type "Vector Structure") (PointTwo :type "Vector Structure"))
  (returns (NewPosition :type "Vector Structure"))
  (return (`KismetMathLibrary.MakeVector` (.x (* (`KismetMathLibrary.Normal` (- PointOne PointTwo)) (`self.AbilityRange`))) (.y (* (`KismetMathLibrary.Normal` (- PointOne PointTwo)) (`self.AbilityRange`))) (+ (.z (* (`KismetMathLibrary.Normal` (- PointOne PointTwo)) (`self.AbilityRange`))) 1.0))))

(fn `UpdatePosition`
  (bind _asthird_person_character (cast `/Game/ThirdPersonBP/Blueprints/ThirdPersonCharacter` (`GameplayStatics.GetPlayerCharacter` 0)))
  (`self.K2_SetActorTransform` (`KismetMathLibrary.MakeTransform` (`KismetMathLibrary.MakeVector` (.x (+ (`self.K2_GetActorLocation` _asthird_person_character) (`KismetMathLibrary.GetForwardVector` (`Pawn.GetControlRotation` _asthird_person_character)))) (.y (+ (`self.K2_GetActorLocation` _asthird_person_character) (`KismetMathLibrary.GetForwardVector` (`Pawn.GetControlRotation` _asthird_person_character)))) (+ (.z (+ (`self.K2_GetActorLocation` _asthird_person_character) (`KismetMathLibrary.GetForwardVector` (`Pawn.GetControlRotation` _asthird_person_character)))) 1.0)) (struct) (`self.GetActorScale3D`))))

(fn `UserConstructionScript`)