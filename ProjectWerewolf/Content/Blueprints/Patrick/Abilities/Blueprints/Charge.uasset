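; Charge ability actor that shows an arrow indicator in front of player 0's character while aiming.
; Left click, when grounded, removes the arrow, sets the cooldown and calls ServerCharge; right click cancels.
; Tick keeps the actor ahead of the character and, once cast, sends mesh overlaps to ServerDamage.
; It zeroes velocity if airborne, and after a short delay stops the character and destroys itself.
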(event `self.ReceiveBeginPlay`
  ;[1 1 1] Spawn Effect
  (bind _returnvalue (`GameplayStatics.SpawnEmitterAtLocation` "/Game/Blueprints/Patrick/Abilities/ParticleSystems/Arrow.Arrow" (.location (`self.GetTransform`)) (.rotation (`self.GetTransform`)) (.scale (`self.GetTransform`)) false))
  (set `self.VisualEmitter` _returnvalue))

(event `Key|LeftMouseButton`
  (params (Key :type "Key Structure"))
  (bind _asthird_person_character (cast `/Game/ThirdPersonBP/Blueprints/ThirdPersonCharacter` (`GameplayStatics.GetPlayerCharacter` 0) :!pure true))
  (:`Pressed`
    ;[1 1 1] Cancel / Cast
    (if (`NavMovementComponent.IsMovingOnGround` (`Character.CharacterMovement` (cast `/Game/ThirdPersonBP/Blueprints/ThirdPersonCharacter` (`GameplayStatics.GetPlayerCharacter` 0) :!pure true)))
      (`self.CleanUp`)
      (set `self.IsCasted?` true)
      (`/Game/Blueprints/Patrick/Abilities/Blueprints/AbilitySystem.SetCooldown` (`/Game/ThirdPersonBP/Blueprints/ThirdPersonCharacter.AbilitySystem` _asthird_person_character) (`self.Cooldown`))
      (`/Game/ThirdPersonBP/Blueprints/ThirdPersonCharacter.ServerCharge` _asthird_person_character (`self.ChargeLength`)))))

(event `Key|RightMouseButton`
  (params (Key :type "Key Structure"))
  ;[1 1 1] Cancel / Cast
  (:`Pressed`
    (`/Game/Blueprints/Patrick/Abilities/Blueprints/AbilitySystem.CancelAbility` (`/Game/ThirdPersonBP/Blueprints/ThirdPersonCharacter.AbilitySystem` (cast `/Game/ThirdPersonBP/Blueprints/ThirdPersonCharacter` (`GameplayStatics.GetPlayerCharacter` 0) :!pure true)))
    (`self.CleanUp`)
    (`self.K2_DestroyActor`)))

(event `self.ReceiveActorBeginOverlap`
  (params (OtherActor :type "Actor Object Reference")))

(event `self.ReceiveTick`
  (params (DeltaSeconds :type "Float (single-precision)"))
  (bind _asthird_person_character (cast `/Game/ThirdPersonBP/Blueprints/ThirdPersonCharacter` (`GameplayStatics.GetPlayerCharacter` 0) :!pure true))
  (bind _charactermovement (`Character.CharacterMovement` _asthird_person_character))
  ;[1 1 1] Update
  (if (`self.IsCasted?`)
    (if (not (`NavMovementComponent.IsMovingOnGround` _charactermovement))
      (set `MovementComponent.Velocity` (0.0 0.0 0.0) _charactermovement))
    (`self.UpdatePosition`)
    (`/Game/Blueprints/Patrick/Abilities/Blueprints/AbilitySystem.Server_damage` (`/Game/ThirdPersonBP/Blueprints/ThirdPersonCharacter.AbilitySystem` _asthird_person_character) _asthird_person_character (`PrimitiveComponent.GetOverlappingActors` (`self.StaticMesh`) "/Script/Engine.Actor") (`self.Damage`))
    (`KismetSystemLibrary.Delay` 0.3)
    (set `MovementComponent.Velocity` (0.0 0.0 0.0) _charactermovement)
    (`self.K2_DestroyActor`)
    (else
      (`self.UpdatePosition`))))

(fn `CleanUp`
  (`ActorComponent.K2_DestroyComponent` (`self.VisualEmitter`)))

(fn `MaxLocation`
  (params (PointOne :type "Vector Structure") (PointTwo :type "Vector Structure"))
  (returns (NewPosition :type "Vector Structure"))
  (return (`KismetMathLibrary.MakeVector` (.x (* (`KismetMathLibrary.Normal` (- PointOne PointTwo)) (`self.AbilityRange`))) (.y (* (`KismetMathLibrary.Normal` (- PointOne PointTwo)) (`self.AbilityRange`))) (+ (.z (* (`KismetMathLibrary.Normal` (- PointOne PointTwo)) (`self.AbilityRange`))) 1.0))))

(fn `UpdatePosition`
  (bind _asthird_person_character (cast `/Game/ThirdPersonBP/Blueprints/ThirdPersonCharacter` (`GameplayStatics.GetPlayerCharacter` 0) :!pure true))
  (bind _returnvalue (`KismetMathLibrary.MakeTransform` (`KismetMathLibrary.MakeVector` (.x (+ (* (`KismetMathLibrary.Normal` (`self.GetActorForwardVector` _asthird_person_character)) 200) (.location (`self.GetTransform` _asthird_person_character)))) (.y (+ (* (`KismetMathLibrary.Normal` (`self.GetActorForwardVector` _asthird_person_character)) 200) (.location (`self.GetTransform` _asthird_person_character)))) (- (.z (+ (* (`KismetMathLibrary.Normal` (`self.GetActorForwardVector` _asthird_person_character)) 200) (.location (`self.GetTransform` _asthird_person_character)))) 98.0)) (`KismetMathLibrary.MakeRotator` (.roll (.rotation (`self.GetTransform` _asthird_person_character))) (.pitch (.rotation (`self.GetTransform` _asthird_person_character))) (+ (.yaw (.rotation (`self.GetTransform` _asthird_person_character))) 180.0)) (1.5 1.5 1.0)))
  (`self.K2_SetActorTransform` _returnvalue)
  (if (not (`self.IsCasted?`))
    (`SceneComponent.K2_SetWorldTransform` (`self.VisualEmitter`) _returnvalue false false)))

(fn `UserConstructionScript`)