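; BuiltStructure is a Blueprint for placing structures on landscape terrain through player input.
; Pressing B enters build mode, traces forward from the player along control rotation, and spawns SelectedStructure on a landscape hit, aligned to the surface normal.
; While building, Tick sets CanBuild by checking CurrentStructure for overlapping actors, though CurrentStructure is never assigned here.
; Left click calls ClearData when building is allowed, but that function is empty.
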(event `Key|LeftMouseButton`
  (params (Key :type "Key Structure"))
  (:`Pressed`
    (if (`self.CanBuild`)
      (`self.ClearData`))))

(event `Key|B`
  (params (Key :type "Key Structure"))
  (bind _returnvalue (`GameplayStatics.GetPlayerCharacter` 0))
  (bind _returnvalue_2 (`self.K2_GetActorLocation` _returnvalue))
  (:`Pressed`
    (set `self.IsBuilding` true)
    (bind _outhit (`KismetSystemLibrary.LineTraceSingle` :`Start` _returnvalue_2 :`End` (+ _returnvalue_2 (* (`KismetMathLibrary.GetForwardVector` (`Pawn.GetControlRotation` _returnvalue)) 500.0)) :`TraceChannel` "TraceTypeQuery1" :`DrawDebugType` "ForDuration"))
    (bind (_bblockinghit _binitialoverlap _time _distance _location _impactpoint _normal _impactnormal _physmat _hitactor) (`GameplayStatics.BreakHitResult` _outhit))
    (if _bblockinghit
      (cast `Landscape` _hitactor)
      (`|SpawnActorFromClass` (`GameplayStatics.GetObjectClass` (`self.SelectedStructure`)) (`KismetMathLibrary.MakeTransform` (`KismetMathLibrary.MakeVector` (.x _location) (.y _location) (.z _location)) (`KismetMathLibrary.MakeRotFromZ` _normal) (100.0 100.0 100.0)) "Undefined" "OverrideRootScale" null null))))

(event `self.ReceiveTick`
  (params (DeltaSeconds :type "Float (single-precision)"))
  (if (`self.IsBuilding`)
    (`self.CheckOverlapping`)))

(fn `CheckOverlapping`
  (if (> (`KismetArrayLibrary.Array_Length` (`self.GetOverlappingActors` (`self.CurrentStructure`) "/Script/Engine.Actor")) 0)
    (set `self.CanBuild` false :!label _label)
    (elif (> (`KismetArrayLibrary.Array_Length` (`self.GetOverlappingActors` (`self.CurrentStructure`) "/Script/Engine.StaticMeshActor")) 0)
      (goto _label)
      (else
        (set `self.CanBuild` true)))))

(fn `ClearData`)

(fn `UserConstructionScript`)